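; Pistol projectile actor that damages a platform game character on impact and destroys itself when its lifespan delay runs out.
; On hitting a BP_PlatformGameCharacter, it calls RegisterHit with damage and an impact velocity opposite its forward vector, then plays a hit montage on that character's mesh.
; Any hit plays a bullet impact sound at the hit location and destroys the projectile.
; OnReset also destroys it.
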(event EventOnReset
  (Actor|DestroyActor))

(event Collision|EventHit
  (params (MyComp :type Primitive%20Component%20Object%20Reference) (Other :type Actor%20Object%20Reference) (OtherComp :type Primitive%20Component%20Object%20Reference) (bSelfMoved :type Boolean) (HitLocation :type Vector :default "0, 0, 0") (HitNormal :type Vector :default "0, 0, 0") (NormalImpulse :type Vector :default "0, 0, 0") (Hit :type Hit%20Result%20Structure%20%28by%20ref%29))
  (bind _asbp_platform_game_character (Utilities|Casting|CastToBP_PlatformGameCharacter Other)
    (:then
      (Default|RegisterHit _asbp_platform_game_character (* (Transformation|GetActorForwardVector) (Math|Float|MakeLiteralFloat -1e+03)) (Transformation|GetActorLocation) (Variables|Default|GetDamageDone))
      (Animation|Montage|PlayMontage (Variables|/Script/Engine.Character|GetMesh _asbp_platform_game_character) "/Game/PGTemplate/Blueprints/Characters/Core/Animations/Custom/HitAnim_Anim_Montage.HitAnim_Anim_Montage"
        (:then
          _)))
    (:CastFailed
      _))
  (Audio|PlaySoundatLocation "/Game/PGTemplate/Blueprints/Characters/Enemy/PrototypeWeaponsPack/Sound/Pistol/Pistol_BulletImpact_Cue.Pistol_BulletImpact_Cue" HitLocation "0, 0, 0" 1.0 1.0 0.0 0 0 0 0)
  (Actor|DestroyActor))

(event EventBeginPlay
  (Utilities|FlowControl|Delay (Variables|Default|GetLifeSpan))
  (Utilities|IsValid self
    (:Is%20Valid
      (Actor|DestroyActor))))

(fn ConstructionScript)