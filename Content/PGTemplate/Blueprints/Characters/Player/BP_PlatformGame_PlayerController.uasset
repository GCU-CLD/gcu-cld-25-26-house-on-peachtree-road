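; Player controller for the platform game that handles respawning the player character at its original start point.
; On BeginPlay it stores the pawn's location and attaches the audio listener to the character's mesh, so sound is heard from the character.
; OnReset waits a tick, spawns a new BP_PlayerCharacter at the stored location, adjusting for collisions, then switches the view target to it and possesses it.
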(event EventBeginPlay
  (bind _returnvalue (Pawn|GetControlledPawn))
  (Variables|Default|SetPlayerSpawnLocation (Transformation|GetActorLocation _returnvalue))
  (Class|PlayerController|SetAudioListenerOverride (Variables|/Script/Engine.Character|GetMesh (.AsBP%20Platform%20Game%20Character (Utilities|Casting|CastToBP_PlatformGameCharacter _returnvalue))) "0, 0, 0" "0, 0, 0"))

(event EventOnReset
  (Utilities|FlowControl|DelayUntilNextTick)
  (bind _returnvalue (Game|SpawnActorfromClass "/Game/PGTemplate/Blueprints/Characters/Player/BP_PlayerCharacter.BP_PlayerCharacter_C" (Math|Transform|MakeTransform (Variables|Default|GetPlayerSpawnLocation) "0, 0, 0" "1.000000,1.000000,1.000000") "AdjustIfPossibleButAlwaysSpawn" "MultiplyWithRoot" 0 0))
  (Game|Player|SetViewTargetwithBlend _returnvalue 0.0 "VTBlend_Linear" 0.0 false)
  (Pawn|Possess _returnvalue))

(fn ConstructionScript)