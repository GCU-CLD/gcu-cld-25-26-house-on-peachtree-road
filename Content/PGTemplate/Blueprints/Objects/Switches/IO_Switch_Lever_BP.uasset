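; Lever switch interactable that a character pulls to toggle its on/off state.
; On interact, it blocks character control, crouches the character if the hand anchor is too low, and plays a left or right grip montage based on facing.
; A timeline swings the lever while driving the character's matching hand anchor to the lever end, then restores control and toggles the switch.
; Reset snaps lever and timeline to the current state.
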(event EventBeginPlay
  (|CallParentFunction) ; This node is disabled and will not be called.\nDrag off pins to build functionality.
)

(event Collision|EventActorBeginOverlap
  (params (OtherActor :type Actor%20Object%20Reference))
  (|CallParentFunction OtherActor) ; This node is disabled and will not be called.\nDrag off pins to build functionality.
)

(event EventTick
  (params (DeltaSeconds :type Float%20%28single-precision%29))
  (|CallParentFunction DeltaSeconds) ; This node is disabled and will not be called.\nDrag off pins to build functionality.
)

(event EventInteract
  (params (InstigatingCharacter :type BP%20Platform%20Game%20Character%20Object%20Reference))
  (bind _returnvalue (Transformation|GetActorRotation InstigatingCharacter))
  (bind _leverend (Variables|Default|GetLeverEnd))
  (bind _returnvalue_2 (Transformation|GetWorldLocation _leverend))
  (bind _returnvalue_3 (Math|Float|Absolute(Float) (.yaw _returnvalue)))
  (bind _returnvalue_4 (> _returnvalue_3 9e+01))
  (if (> (- (.z (Transformation|GetActorLocation InstigatingCharacter)) (.z (Transformation|GetWorldLocation (Variables|Default|GetHandAnchor)))) 5e+01)
    (Character|Crouch InstigatingCharacter))
  (Default|BlockControl InstigatingCharacter false)
  (Animation|PlayAnimMontage InstigatingCharacter (select _returnvalue_4 "/Game/PGTemplate/Blueprints/Characters/Core/Animations/Mixamo/Interactions/ButtonPushing_R_Grip_UE_Montage.ButtonPushing_R_Grip_UE_Montage" "/Game/PGTemplate/Blueprints/Characters/Core/Animations/Mixamo/Interactions/ButtonPushing_L_Grip_UE_Montage.ButtonPushing_L_Grip_UE_Montage") 3.0 "None")
  (if (Variables|Default|GetSwitchIsOn)
    (bind _leverrotation (Timeline|Timeline Reverse)
      (:Update
        (Transformation|SetRelativeRotation (Variables|Default|GetLeverRoot) (Math|Rotator|MakeRotator (* _leverrotation 4e+01) 0.0 0.0) false false)
        (if _returnvalue_4
          (Variables|/Game/PGTemplate/Blueprints/Characters/Player/BP_PlayerCharacter.BP_PlayerCharacter_C|SetHandAnchorRight InstigatingCharacter _returnvalue_2)
          (else
            (Variables|/Game/PGTemplate/Blueprints/Characters/Player/BP_PlayerCharacter.BP_PlayerCharacter_C|SetHandAnchorLeft InstigatingCharacter _returnvalue_2))))
      (:Finished
        (Default|UnBlockControl InstigatingCharacter)
        (CallFunction|ToggleSwitchStatus)))
    (else
      (Timeline|Timeline Play))))

(event EventOnReset
  (bind _switchison (Variables|Default|GetSwitchIsOn))
  (bind _timeline (Variables|Default|GetTimeline))
  (|CallParentFunction)
  (Transformation|SetRelativeRotation (Variables|Default|GetLeverRoot) (Math|Rotator|MakeRotator (Math|Float|SelectFloat 4e+01 -4e+01 _switchison) 0.0 0.0) false false)
  (Components|Timeline|SetPlaybackPosition _timeline (Math|Float|SelectFloat (Components|Timeline|GetTimelineLength _timeline) 0.0 _switchison) false false))

(fn ConstructionScript
  (|CallParentFunction)
  (Transformation|AttachComponentToComponent (Variables|Default|GetLeverEnd) (Variables|Default|GetCylinder_0) "None" "KeepRelative" "KeepRelative" "KeepRelative" true))