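; IO_Slot_BP is an interactable slot switch that turns on while it holds an object of the required class.
; Interacting inserts a matching carried object or hands the slotted one back; otherwise the character briefly loses control and plays a head-shake montage.
; Slotting disables physics and snaps the mesh to SlotInput, and each state change updates the indicator and targeted actors.
; It can spawn pre-filled, and reset restores that starting state.
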(event Custom|ForceSlotObject
  (params (ObjectToSlot :type Carried%20Object%20IO%20Object%20Reference))
  ;[1 1 1] ForceSlotObject
  (Variables|Default|SetSlottedObejct ObjectToSlot)
  ;[1 1 1] Player Slots Object
  (Physics|SetSimulatePhysics (Variables|/Game/PGTemplate/Blueprints/Objects/Carried/Core/CarriedObject_IO.CarriedObject_IO_C|GetMesh (Variables|Default|GetSlottedObejct)) false)
  (Transformation|AttachComponentToComponent (Variables|/Game/PGTemplate/Blueprints/Objects/Carried/Core/CarriedObject_IO.CarriedObject_IO_C|GetMesh (Variables|Default|GetSlottedObejct)) (Variables|Default|GetSlotInput) "None" "SnapToTarget" "SnapToTarget" "KeepWorld" true)
  (Variables|Default|SetSwitchIsOn true)
  (CallFunction|UpdateIndicator)
  (CallFunction|UpdateTargetedActors))

(event EventBeginPlay
  (|CallParentFunction)
  (if (Variables|Default|GetSpawnSlottedObjectAtStart)
    (bind _returnvalue (Game|SpawnActorfromClass (Variables|Default|GetNecessaryObjectClass) (Math|Transform|MakeTransform (Transformation|GetActorLocation) "0, 0, 0" "1.000000,1.000000,1.000000") "Undefined" "MultiplyWithRoot" 0 0))
    (Variables|Default|SetSpawnedObject _returnvalue)
    (CallFunction|ForceSlotObject _returnvalue)))

(event EventOnReset
  (if (Variables|Default|GetSpawnSlottedObjectAtStart)
    (Actor|DestroyActor (Variables|Default|GetSpawnedObject))
    (bind _returnvalue (Game|SpawnActorfromClass (Variables|Default|GetNecessaryObjectClass) (Math|Transform|MakeTransform (Transformation|GetActorLocation) "0, 0, 0" "1.000000,1.000000,1.000000") "AlwaysSpawn" "MultiplyWithRoot" 0 0))
    (Variables|Default|SetSpawnedObject _returnvalue)
    (Utilities|FlowControl|DelayUntilNextTick)
    (CallFunction|ForceSlotObject (Variables|Default|GetSpawnedObject))
    (CallFunction|UpdateIndicator)
    (CallFunction|UpdateTargetedActors)
    (else
      (Variables|Default|SetSlottedObejct 0)
      (Variables|Default|SetSwitchIsOn false)
      (CallFunction|UpdateIndicator)
      (CallFunction|UpdateTargetedActors)
      (if (Variables|Default|GetSpawnSlottedObjectAtStart)
        (bind _returnvalue_2 (Game|SpawnActorfromClass (Variables|Default|GetNecessaryObjectClass) (Math|Transform|MakeTransform (Transformation|GetActorLocation) "0, 0, 0" "1.000000,1.000000,1.000000") "Undefined" "MultiplyWithRoot" 0 0))
        (Variables|Default|SetSpawnedObject _returnvalue_2)
        (CallFunction|ForceSlotObject _returnvalue_2)))))

(event EventInteract
  (params (InstigatingCharacter :type BP%20Platform%20Game%20Character%20Object%20Reference))
  (bind _currentlycarriedobject (Variables|/Game/PGTemplate/Blueprints/Characters/Core/BP_PlatformGameCharacter.BP_PlatformGameCharacter_C|GetCurrentlyCarriedObject InstigatingCharacter))
  (Utilities|IsValid (Variables|Default|GetSlottedObejct)
    (:Is%20Valid
      ;[1 1 1] Player Removes Slotted Item
      (Default|PickUpNoCrouch (Variables|Default|GetSlottedObejct) InstigatingCharacter)
      (Variables|Default|SetSlottedObejct 0)
      (Variables|Default|SetSwitchIsOn false)
      (CallFunction|UpdateIndicator)
      (CallFunction|UpdateTargetedActors))
    (:Is%20Not%20Valid
      (Utilities|IsValid _currentlycarriedobject
        (:Is%20Valid
          (if (== (Utilities|GetClass _currentlycarriedobject) (Variables|Default|GetNecessaryObjectClass))
            ;[1 1 1] Player Slots Object
            (Variables|Default|SetSlottedObejct _currentlycarriedobject)
            (Default|ForceDrop (Variables|Default|GetSlottedObejct))
            (Physics|SetSimulatePhysics (Variables|/Game/PGTemplate/Blueprints/Objects/Carried/Core/CarriedObject_IO.CarriedObject_IO_C|GetMesh (Variables|Default|GetSlottedObejct)) false)
            (Transformation|AttachComponentToComponent (Variables|/Game/PGTemplate/Blueprints/Objects/Carried/Core/CarriedObject_IO.CarriedObject_IO_C|GetMesh (Variables|Default|GetSlottedObejct)) (Variables|Default|GetSlotInput) "None" "SnapToTarget" "SnapToTarget" "KeepWorld" true)
            (Variables|Default|SetSwitchIsOn true)
            (CallFunction|UpdateIndicator)
            (CallFunction|UpdateTargetedActors)
            (else
              ;[1 1 1] Player Has Incorrect Object
              (Default|BlockControl InstigatingCharacter false :!label _label)
              (bind _returnvalue (Animation|PlayAnimMontage InstigatingCharacter "/Game/PGTemplate/Blueprints/Characters/Core/Animations/Mixamo/Interactions/ThoughtfulHeadShake_UE_Montage.ThoughtfulHeadShake_UE_Montage" 2.0 "None"))
              (Utilities|FlowControl|Delay (/ _returnvalue 2.0))
              (Default|UnBlockControl InstigatingCharacter))))
        (:Is%20Not%20Valid
          (goto _label))))))

(fn ConstructionScript
  (|CallParentFunction))