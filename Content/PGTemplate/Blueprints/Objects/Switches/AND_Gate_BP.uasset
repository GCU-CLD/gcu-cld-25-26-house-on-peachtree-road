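; AND gate switch that counts as on only when every switch targeting it is on, then updates its own targeted actors.
; One tick after BeginPlay it finds those switches through the GameMode's AllSwitchesInLevel list and prints a warning for any missing from IndicatorOrder.
; The construction script builds a centred row of cylinder indicators from that map, each with a dynamic material.
; Switch on and off events both recolour indicators green or red and re-evaluate the gate.
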(event EventBeginPlay
  (Utilities|FlowControl|DelayUntilNextTick)
  (bind _output_get (Variables|Default|SetTargettingSwitches (CallFunction|GetAllSwitchesTargettingThisActor)))
  (CallFunction|CheckTargettingSwitchesAgainstIndicatorOrder _output_get))

(event EventSwitchon
  (CallFunction|UpdateIndicators)
  (Variables|Default|SetSwitchIsOn (CallFunction|GetOverallSwitchStatus))
  (CallFunction|UpdateTargetedActors))

(event EventSwitchOff
  (CallFunction|UpdateIndicators)
  (Variables|Default|SetSwitchIsOn (CallFunction|GetOverallSwitchStatus))
  (CallFunction|UpdateTargetedActors))

(fn ConstructionScript
  (bind _indicatororder (Variables|Default|GetIndicatorOrder))
  (Utilities|FlowControl|Sequence
    (:then_0
      ;[1 1 1] Create Indicators
      (bind _keys (Utilities|Map|Keys _indicatororder))
      (for (_ _array_index) _keys
        (bind _keys_2 (Utilities|Map|Keys _indicatororder))
        (for _array_element _keys_2
          (if (== (.Value (Utilities|Map|Find (Variables|Default|GetIndicatorOrder) _array_element)) _array_index)
            (bind _returnvalue (AddComponent|AddStaticMeshComponent false (Math|Transform|MakeTransform (Math|Vector|MakeVector (Math|Conversions|ToFloat(Integer) (- (* _array_index 60) (/ (* (- (Utilities|Array|Length _keys) 1) 60) 2))) 0.0 0.0) "0.000000,0.000000,90.000000" "0.500000,0.500000,0.100000")))
            (Components|StaticMesh|SetStaticMesh _returnvalue "/Engine/BasicShapes/Cylinder.Cylinder")
            (bind _returnvalue_2 (Rendering|Material|CreateDynamicMaterialInstance "/Game/PGTemplate/Environments/Materials/BasicColouredMaterial_M.BasicColouredMaterial_M" "None" "None" :!class /Script/Engine.KismetMaterialLibrary))
            (Rendering|Material|SetMaterial _returnvalue 0 _returnvalue_2)
            (Utilities|Map|Add (Variables|Default|GetSwitchesAndMaterials) _array_element _returnvalue_2)))))
    (:then_1
      (CallFunction|UpdateIndicators))))

(fn GetAllSwitchesTargettingThisActor
  (for _array_element (Variables|/Game/PGTemplate/Blueprints/Core/BP_PlatformGame_GameMode.BP_PlatformGame_GameMode_C|GetAllSwitchesInLevel (.AsBP%20Platform%20Game%20Game%20Mode (Utilities|Casting|CastToBP_PlatformGame_GameMode (Game|GetGameMode))))
    (for _array_element_2 (Variables|/Game/PGTemplate/Blueprints/Objects/Switches/IO_Switch_BP.IO_Switch_BP_C|GetTargetedActors _array_element)
      (if (== _array_element_2 self)
        (Utilities|Array|Add (LocalVariables|GetFoundSwitchesLocal) _array_element))))
  (return (LocalVariables|GetFoundSwitchesLocal)))

(fn CheckTargettingSwitchesAgainstIndicatorOrder
  (params (Array :type Array%20of%20IO%20Switch%20BP%20Object%20References))
  (for _array_element Array
    (if (not (.ReturnValue (Utilities|Map|Find (Variables|Default|GetIndicatorOrder) _array_element)))
      (Development|PrintString (Utilities|String|Append "Switch " (Utilities|GetDisplayName _array_element) " targets AND_Gate " (Utilities|GetDisplayName self) " but is not present in the Indicator Order map")))))

(fn GetStatus
  (return (CallFunction|GetOverallSwitchStatus)))

(fn UpdateIndicators
  (bind _switchesandmaterials (Variables|Default|GetSwitchesAndMaterials))
  (bind _keys (Utilities|Map|Keys _switchesandmaterials))
  (for _array_element _keys
    (Rendering|Material|SetVectorParameterValue (.Value (Utilities|Map|Find _switchesandmaterials _array_element)) "Colour" (Math|Color|SelectColor "(R=0.000000,G=1.000000,B=0.000000,A=1.000000)" "(R=1.000000,G=0.000000,B=0.000000,A=1.000000)" (Variables|/Game/PGTemplate/Blueprints/Objects/Switches/IO_Switch_BP.IO_Switch_BP_C|GetSwitchIsOn _array_element)) :!class /Script/Engine.MaterialInstanceDynamic)))

(fn GetOverallSwitchStatus
  (LocalVariables|SetLocalOverallSwitchIsOn true)
  (for _array_element (Variables|Default|GetTargettingSwitches)
    (if (not (Variables|/Game/PGTemplate/Blueprints/Objects/Switches/IO_Switch_BP.IO_Switch_BP_C|GetSwitchIsOn _array_element))
      (LocalVariables|SetLocalOverallSwitchIsOn false)))
  (return (LocalVariables|GetLocalOverallSwitchIsOn)))