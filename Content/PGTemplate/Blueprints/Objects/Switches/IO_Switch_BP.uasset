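; Interactable switch that toggles on/off and relays its state to a list of targeted actors through on/off and initial-status messages.
; Interacting plays a left or right button-push montage chosen by character yaw, setting hand anchors, crouching if needed and blocking control.
; After the animation, it toggles state and recolours a dynamic-material indicator.
; Construction, BeginPlay and reset apply the initial state to indicator and targets.
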(event Custom|PostSwitchActions
  (params (InstigatingCharacter :type BP%20Platform%20Game%20Character%20Object%20Reference)))

(event EventBeginPlay
  (Variables|Default|SetSwitchIsOn (Variables|Default|GetInitialState))
  (CallFunction|UpdateIndicator)
  (CallFunction|SetInitialStateonTargetedActors))

(event EventOnReset
  (Variables|Default|SetSwitchIsOn (Variables|Default|GetInitialState))
  (CallFunction|UpdateIndicator)
  (CallFunction|SetInitialStateonTargetedActors))

(event EventInteract
  (params (InstigatingCharacter :type BP%20Platform%20Game%20Character%20Object%20Reference))
  (|CallParentFunction InstigatingCharacter)
  (|ButtonPushingAnimation InstigatingCharacter
    (:Out
      (CallFunction|PostSwitchActions InstigatingCharacter)
      (CallFunction|ToggleSwitchStatus))))

(fn ConstructionScript
  (|CallParentFunction)
  (Transformation|SetRelativeLocation (Variables|Default|GetHandAnchor) (Variables|Default|GetHandAnchorPosition) false false)
  (Variables|Default|SetSwitchIsOn (Variables|Default|GetInitialState))
  (bind _returnvalue (Rendering|Material|CreateDynamicMaterialInstance "/Game/PGTemplate/Blueprints/Objects/Switches/Materials/SwitchIndicator_M.SwitchIndicator_M" "None" "None" :!class /Script/Engine.KismetMaterialLibrary))
  (bind _output_get (Variables|Default|SetIndicatorMaterial _returnvalue))
  (Rendering|Material|SetMaterial (Variables|Default|GetStatusIndicator) 0 _output_get)
  (CallFunction|UpdateIndicator)
  (CallFunction|UpdateTargetedActors))

(fn UpdateTargetedActors
  (for _array_element (Variables|Default|GetTargetedActors)
    (if (Variables|Default|GetSwitchIsOn)
      (Class|SwitchInterface|Switchon(Message) _array_element)
      (else
        (Class|SwitchInterface|SwitchOff(Message) _array_element)))))

(fn UpdateIndicator
  (bind _indicatormaterial (Variables|Default|GetIndicatorMaterial))
  (Utilities|IsValid _indicatormaterial
    (:Is%20Valid
      (Rendering|Material|SetVectorParameterValue _indicatormaterial "Colour" (Math|Color|SelectColor (Variables|Default|GetOnColour) (Variables|Default|GetOffColour) (Variables|Default|GetSwitchIsOn)) :!class /Script/Engine.MaterialInstanceDynamic))))

(fn ToggleSwitchStatus
  (if (Variables|Default|GetSwitchIsOn)
    (Variables|Default|SetSwitchIsOn false)
    (else
      (Variables|Default|SetSwitchIsOn true)))
  (CallFunction|UpdateIndicator)
  (CallFunction|UpdateTargetedActors))

(fn SetInitialStateonTargetedActors
  (for _array_element (Variables|Default|GetTargetedActors)
    (Class|SwitchInterface|SetInitialStatus(Message) _array_element (Variables|Default|GetSwitchIsOn))))

(fn GetStatus
  (return false))