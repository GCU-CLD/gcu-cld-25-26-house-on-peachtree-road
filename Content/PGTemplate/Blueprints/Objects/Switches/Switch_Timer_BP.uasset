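; Timed switch actor that, on interaction, turns on after a delay, then off after another, updating its targeted actors each time.
; Interact first plays a side-dependent button-press montage on the character, with hand anchoring, blocked control and a crouch for low switches.
; The MaterialCompletion timeline then plays forward and backward, rate-scaled to each delay.
; The construction script gives StatusIndicator a dynamic material with on/off colours and a Completion parameter for progress.
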(event EventBeginPlay
  (|CallParentFunction) ; This node is disabled and will not be called.\nDrag off pins to build functionality.
)

(event Collision|EventActorBeginOverlap
  (params (OtherActor :type Actor%20Object%20Reference))
  (|CallParentFunction OtherActor) ; This node is disabled and will not be called.\nDrag off pins to build functionality.
)

(event EventTick
  (params (DeltaSeconds :type Float%20%28single-precision%29))
  (|CallParentFunction DeltaSeconds) ; This node is disabled and will not be called.\nDrag off pins to build functionality.
)

(event EventInteract
  (params (InstigatingCharacter :type BP%20Platform%20Game%20Character%20Object%20Reference))
  (bind _materialcompletion (Variables|Default|GetMaterialCompletion))
  (bind _materialcompletion_2 (Variables|Default|GetMaterialCompletion))
  (|CollapseGraph_2 InstigatingCharacter
    (:Out
      (Components|Timeline|SetPlayRate _materialcompletion_2 (/ 1.0 (Variables|Default|GetDelayBeforeOn)))
      (Components|Timeline|PlayfromStart _materialcompletion_2)
      (Utilities|FlowControl|Delay (Variables|Default|GetDelayBeforeOn))
      (Variables|Default|SetSwitchIsOn true)
      (CallFunction|UpdateTargetedActors)
      (Components|Timeline|SetPlayRate _materialcompletion (/ 1.0 (Variables|Default|GetDelayBeforeOff)))
      (Components|Timeline|ReversefromEnd _materialcompletion)
      (Utilities|FlowControl|Delay (Variables|Default|GetDelayBeforeOff))
      (Variables|Default|SetSwitchIsOn false)
      (CallFunction|UpdateTargetedActors))))

(fn ConstructionScript
  (|CallParentFunction)
  (bind _returnvalue (Rendering|Material|CreateDynamicMaterialInstance "/Game/PGTemplate/Blueprints/Objects/Switches/Materials/Timer_M.Timer_M" "None" "None" :!class /Script/Engine.KismetMaterialLibrary))
  (bind _output_get (Variables|Default|SetTimerMaterial _returnvalue))
  (Rendering|Material|SetMaterial (Variables|Default|GetStatusIndicator) 0 _output_get)
  (Rendering|Material|SetVectorParameterValue (Variables|Default|GetTimerMaterial) "OnColour" (Variables|Default|GetOnColour) :!class /Script/Engine.MaterialInstanceDynamic)
  (Rendering|Material|SetVectorParameterValue (Variables|Default|GetTimerMaterial) "OffColour" (Variables|Default|GetOffColour) :!class /Script/Engine.MaterialInstanceDynamic)
  (Rendering|Material|SetScalarParameterValue (Variables|Default|GetTimerMaterial) "Completion" 0.0 :!class /Script/Engine.MaterialInstanceDynamic))