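; Camera switch that turns off while it sees the player, or optionally an enemy, and updates its indicator and targeted actors; OppositeMode inverts this.
; A fan of visibility line traces defines its view and shapes a dynamic vision mesh built in construction.
; Tick rebuilds vertices and re-evaluates detection only when hits change, with paired DoOnce nodes limiting state and cone colour updates to transitions.
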(event EventBeginPlay
  (|CallParentFunction)
  (Variables|Default|SetLastHitResults (.HitResults (CallFunction|CameraLineTraces)))
  (Rendering|Material|SetVectorParameterValue (Variables|Default|GetVisionMaterial) "None" (Math|Color|SelectColor (Variables|Default|GetOnColour) (Variables|Default|GetOffColour) (Variables|Default|GetSwitchIsOn)) :!class /Script/Engine.MaterialInstanceDynamic))

(event Collision|EventActorBeginOverlap
  (params (OtherActor :type Actor%20Object%20Reference))
  (|CallParentFunction OtherActor) ; This node is disabled and will not be called.\nDrag off pins to build functionality.
)

(event EventTick
  (params (DeltaSeconds :type Float%20%28single-precision%29))
  (bind _oppositemode (Variables|Default|GetOppositeMode))
  (|CallParentFunction DeltaSeconds)
  (Utilities|FlowControl|Sequence
    (:then_0
      ;[1 1 1] If Hit Results have changed since last update ...
      (bind _output_get (Variables|Default|SetNewHitResults (.HitResults (CallFunction|CameraLineTraces))))
      (if (not (Utilities|Array|Identical _output_get (Variables|Default|GetLastHitResults)))
        ;[1 1 1] ... then redraw the mesh!
        (bind _returnvalue (DynamicMeshComponent|GetDynamicMesh (Variables|Default|GetVisionMesh)))
        (bind _vectorlist (GeometryScript|ListUtils|ConvertArraytoVectorList (CallFunction|HitResultstoVectorPoints (Variables|Default|GetNewHitResults) (Transformation|GetActorLocation) (Transformation|GetActorRotation))))
        (Class|GeometryScriptLibraryMeshBasicEditFunctions|SetAllMeshVertexPositions _returnvalue _vectorlist 0)
        (Variables|Default|SetTriggered false)
        (for _array_element (Variables|Default|GetNewHitResults)
          (Utilities|Casting|CastToBP_PlayerCharacter (.hitactor _array_element)
            (:then
              (Variables|Default|SetTriggered true))
            (:CastFailed
              (if (Variables|Default|GetTriggeredByEnemies)
                (Utilities|Casting|CastToBP_Enemy_Base (.hitactor _array_element))
                (Variables|Default|SetTriggered true)))))
        (if (Variables|Default|GetTriggered)
          (if _oppositemode
            (Utilities|FlowControl|Sequence :!label _label
              (:then_0
                (Utilities|FlowControl|DoOnce false :!label _label_2
                  (:Completed
                    (Variables|Default|SetSwitchIsOn true)
                    (Rendering|Material|SetVectorParameterValue (Variables|Default|GetVisionMaterial) "Colour" (Variables|Default|GetOnColour) :!class /Script/Engine.MaterialInstanceDynamic)
                    (CallFunction|UpdateIndicator)
                    (CallFunction|UpdateTargetedActors))))
              (:then_1
                (goto _label_4 Reset)))
            (else
              (Utilities|FlowControl|Sequence :!label _label_3
                (:then_0
                  (Utilities|FlowControl|DoOnce false :!label _label_4
                    (:Completed
                      (Variables|Default|SetSwitchIsOn false)
                      (Rendering|Material|SetVectorParameterValue (Variables|Default|GetVisionMaterial) "Colour" (Variables|Default|GetOffColour) :!class /Script/Engine.MaterialInstanceDynamic)
                      (CallFunction|UpdateIndicator)
                      (CallFunction|UpdateTargetedActors))))
                (:then_1
                  (goto _label_2 Reset)))))
          (elif _oppositemode
            (goto _label_3)
            (else
              (goto _label))))))
    (:then_1
      ;[1 1 1] Store Hit Results for next update
      (Variables|Default|SetLastHitResults (Variables|Default|GetNewHitResults)))))

(fn ConstructionScript
  (Variables|Default|SetInitialState (not (Variables|Default|GetOppositeMode)))
  (|CallParentFunction)
  (Utilities|FlowControl|Sequence
    (:then_0
      ;[1 1 1] Build Vertices and Triangles for the Vision Mesh
      (bind _returnvalue (DynamicMeshComponent|GetDynamicMesh (Variables|Default|GetVisionMesh)))
      (Class|GeometryScriptLibraryMeshBasicEditFunctions|AddVertextoMesh _returnvalue "0, 0, 0" false)
      (LocalVariables|SetInitialHits (.HitResults (CallFunction|CameraLineTraces)))
      (for _array_element (LocalVariables|GetInitialHits)
        (bind _returnvalue_2 (DynamicMeshComponent|GetDynamicMesh (Variables|Default|GetVisionMesh)))
        (Class|GeometryScriptLibraryMeshBasicEditFunctions|AddVertextoMesh _returnvalue_2 (Math|Vector|UnrotateVector (- (Math|Vector|SelectVector (.ImpactPoint (Collision|BreakHitResult _array_element)) (.TraceEnd (Collision|BreakHitResult _array_element)) (.bBlockingHit (Collision|BreakHitResult _array_element))) (Transformation|GetActorLocation)) (Transformation|GetActorRotation)) false))
      (for _index (range 0 (- (Utilities|Array|Length (LocalVariables|GetInitialHits)) 2))
        (bind _returnvalue_3 (DynamicMeshComponent|GetDynamicMesh (Variables|Default|GetVisionMesh)))
        (GeometryScript|MeshEdits|AddTriangletoMesh _returnvalue_3 (Utilities|Struct|MakeIntVector 0 (+ _index 2) (+ _index 1)) 0 false 0)))
    (:then_1
      (bind _returnvalue_4 (Rendering|Material|CreateDynamicMaterialInstance "/Game/PGTemplate/Blueprints/Objects/Switches/Materials/CameraVisionCone_M.CameraVisionCone_M" "None" "None" :!class /Script/Engine.KismetMaterialLibrary))
      (bind _output_get (Variables|Default|SetVisionMaterial _returnvalue_4))
      (Rendering|Material|SetMaterial (Variables|Default|GetVisionMesh) 0 _output_get)
      (Rendering|Material|SetVectorParameterValue (Variables|Default|GetVisionMaterial) "Colour" (Math|Color|SelectColor (Variables|Default|GetOffColour) (Variables|Default|GetOnColour) (Variables|Default|GetOppositeMode)) :!class /Script/Engine.MaterialInstanceDynamic))))

(fn CameraLineTraces
  (bind _returnvalue (Transformation|GetActorLocation))
  (bind _visionangle (Variables|Default|GetVisionAngle))
  (bind _returnvalue_2 (/ _visionangle 2.0))
  (Utilities|Array|Clear (LocalVariables|GetHitResultsLocal))
  (LocalVariables|SetBlockingHitFoundLocal false)
  (for _index (range 0 (Math|Float|Ceil (/ (Variables|Default|GetVisionAngle) (Variables|Default|GetVisionTestAngle))))
    (bind (_outhit _returnvalue_3) (Collision|LineTraceByChannel _returnvalue (+ _returnvalue (Math|Vector|RotateVectorAroundAxis (* (Math|Vector|RotateVectorAroundAxis (Transformation|GetActorForwardVector) 9e+01 "0.000000,1.000000,0.000000") (Variables|Default|GetVisionDistance)) (Math|Float|Clamp(Float) (- (* _index (Variables|Default|GetVisionTestAngle)) _returnvalue_2) (* _returnvalue_2 -1.0) _returnvalue_2) "0.000000,1.000000,0.000000")) "TraceTypeQuery1" false 0 "None"))
    (if _returnvalue_3
      (LocalVariables|SetBlockingHitFoundLocal true))
    (Utilities|Array|Add (LocalVariables|GetHitResultsLocal) _outhit))
  (return (LocalVariables|GetHitResultsLocal) (LocalVariables|GetBlockingHitFoundLocal)))

(fn HitResultstoVectorPoints
  (params (HitResults :type Array%20of%20Hit%20Result%20Structures) (ActorLocation :type Vector) (ActorRotation :type Rotator))
  (bind _outputverts (LocalVariables|GetOutputVerts))
  (Utilities|Array|Clear _outputverts)
  (Utilities|Array|Add :TargetArray _outputverts)
  (for _array_element HitResults
    (Utilities|Array|Add (LocalVariables|GetOutputVerts) (Math|Vector|UnrotateVector (- (Math|Vector|SelectVector (.impactpoint _array_element) (.traceend _array_element) (.bblockinghit _array_element)) ActorLocation) (Transformation|GetActorRotation))))
  (return (LocalVariables|GetOutputVerts)))