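; Pressure plate switch that turns on while an actor tagged "Weight" overlaps its box and off otherwise.
; Each box begin or end overlap rechecks the overlapping actors, sets the switch state, and calls updates for the indicator and targeted actors.
; The same event plays a sound and drives a timeline that moves the plate along Z, reversing it when unweighted.
; The construction script colours the plate through a dynamic material instance.
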(event OnComponentBeginOverlap(Box)
  (params (OverlappedComponent :type Primitive%20Component%20Object%20Reference) (OtherActor :type Actor%20Object%20Reference) (OtherComp :type Primitive%20Component%20Object%20Reference) (OtherBodyIndex :type Integer) (bFromSweep :type Boolean) (SweepResult :type Hit%20Result%20Structure%20%28by%20ref%29))
  (bind _returnvalue (Transformation|GetActorLocation))
  (Variables|Default|SetSwitchIsOn (CallFunction|HasWeight))
  (CallFunction|UpdateIndicator)
  (CallFunction|UpdateTargetedActors)
  (if (CallFunction|HasWeight)
    (Audio|PlaySoundatLocation "/Game/PGTemplate/Blueprints/Characters/Core/Audio/PressurePlate_Cue.PressurePlate_Cue" _returnvalue "0, 0, 0" 1.0 1.0 0.0 0 0 0 0)
    (bind _zoffset (Timeline|PlateMotion Play)
      (:Update
        (Transformation|SetRelativeLocation (Variables|Default|GetPlate) (Math|Vector|MakeVector 0.0 0.0 _zoffset) false false)))
    (else
      (Audio|PlaySoundatLocation "/Game/PGTemplate/Blueprints/Characters/Core/Audio/PressurePlate_Cue.PressurePlate_Cue" _returnvalue "0, 0, 0" 1.0 1.0 0.0 0 0 0 0)
      (Timeline|PlateMotion Reverse))))

(event OnComponentEndOverlap(Box)
  (params (OverlappedComponent :type Primitive%20Component%20Object%20Reference) (OtherActor :type Actor%20Object%20Reference) (OtherComp :type Primitive%20Component%20Object%20Reference) (OtherBodyIndex :type Integer))
  (bind _returnvalue (Transformation|GetActorLocation))
  (Variables|Default|SetSwitchIsOn (CallFunction|HasWeight))
  (CallFunction|UpdateIndicator)
  (CallFunction|UpdateTargetedActors)
  (if (CallFunction|HasWeight)
    (Audio|PlaySoundatLocation "/Game/PGTemplate/Blueprints/Characters/Core/Audio/PressurePlate_Cue.PressurePlate_Cue" _returnvalue "0, 0, 0" 1.0 1.0 0.0 0 0 0 0)
    (bind _zoffset (Timeline|PlateMotion Play)
      (:Update
        (Transformation|SetRelativeLocation (Variables|Default|GetPlate) (Math|Vector|MakeVector 0.0 0.0 _zoffset) false false)))
    (else
      (Audio|PlaySoundatLocation "/Game/PGTemplate/Blueprints/Characters/Core/Audio/PressurePlate_Cue.PressurePlate_Cue" _returnvalue "0, 0, 0" 1.0 1.0 0.0 0 0 0 0)
      (Timeline|PlateMotion Reverse))))

(event EventBeginPlay
  (|CallParentFunction) ; This node is disabled and will not be called.\nDrag off pins to build functionality.
)

(event Collision|EventActorBeginOverlap
  (params (OtherActor :type Actor%20Object%20Reference))
  (|CallParentFunction OtherActor) ; This node is disabled and will not be called.\nDrag off pins to build functionality.
)

(event EventTick
  (params (DeltaSeconds :type Float%20%28single-precision%29))
  (|CallParentFunction DeltaSeconds) ; This node is disabled and will not be called.\nDrag off pins to build functionality.
)

(fn ConstructionScript
  (|CallParentFunction)
  (bind _returnvalue (Rendering|Material|CreateDynamicMaterialInstance "/Game/PGTemplate/Environments/Materials/BasicColouredMaterial_M.BasicColouredMaterial_M" "None" "None" :!class /Script/Engine.KismetMaterialLibrary))
  (bind _output_get (Variables|Default|SetPlateMaterial _returnvalue))
  (Rendering|Material|SetMaterial (Variables|Default|GetPlate) 0 _output_get)
  (Rendering|Material|SetVectorParameterValue (Variables|Default|GetPlateMaterial) "Colour" (Variables|Default|GetPlateColour) :!class /Script/Engine.MaterialInstanceDynamic))

(fn HasWeight
  (LocalVariables|SethasWeightLocal false)
  (for _array_element (Collision|GetOverlappingActors (Variables|Default|GetBox) 0 :!class /Script/Engine.PrimitiveComponent)
    (if (Actor|ActorHasTag _array_element "Weight")
      (LocalVariables|SethasWeightLocal true)))
  (return (LocalVariables|GethasWeightLocal)))