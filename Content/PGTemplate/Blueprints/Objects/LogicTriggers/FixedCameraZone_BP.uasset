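; A trigger zone that switches the view to its own fixed cine camera while the player character is inside.
; On overlap begin it sets OverrideCamera on the platform game camera manager and blends the view target to itself.
; On overlap end it clears the flag and blends back to the controlled pawn over the same BlendTime.
; The construction script resets the camera's world scale to one, independent of actor scaling.
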(event OnComponentBeginOverlap(PlayerDetection)
  (params (OverlappedComponent :type Primitive%20Component%20Object%20Reference) (OtherActor :type Actor%20Object%20Reference) (OtherComp :type Primitive%20Component%20Object%20Reference) (OtherBodyIndex :type Integer) (bFromSweep :type Boolean) (SweepResult :type Hit%20Result%20Structure%20%28by%20ref%29))
  (bind _returnvalue (Game|GetPlayerController 0))
  (Utilities|Casting|CastToBP_PlayerCharacter OtherActor)
  (bind _asbp_platform_game_camera_manager (Utilities|Casting|CastToBP_PlatformGameCameraManager (Variables|/Script/Engine.PlayerController|GetPlayerCameraManager _returnvalue)))
  (Variables|/Game/PGTemplate/Blueprints/Characters/Player/BP_PlatformGameCameraManager.BP_PlatformGameCameraManager_C|SetOverrideCamera _asbp_platform_game_camera_manager true)
  (Game|Player|SetViewTargetwithBlend _returnvalue self (Variables|Default|GetBlendTime) "VTBlend_Linear" 0.0 false))

(event OnComponentEndOverlap(PlayerDetection)
  (params (OverlappedComponent :type Primitive%20Component%20Object%20Reference) (OtherActor :type Actor%20Object%20Reference) (OtherComp :type Primitive%20Component%20Object%20Reference) (OtherBodyIndex :type Integer))
  (bind _returnvalue (Game|GetPlayerController 0))
  (Utilities|Casting|CastToBP_PlayerCharacter OtherActor)
  (bind _asbp_platform_game_camera_manager (Utilities|Casting|CastToBP_PlatformGameCameraManager (Variables|/Script/Engine.PlayerController|GetPlayerCameraManager _returnvalue)))
  (Variables|/Game/PGTemplate/Blueprints/Characters/Player/BP_PlatformGameCameraManager.BP_PlatformGameCameraManager_C|SetOverrideCamera _asbp_platform_game_camera_manager false)
  (Game|Player|SetViewTargetwithBlend _returnvalue (Pawn|GetControlledPawn _returnvalue) (Variables|Default|GetBlendTime) "VTBlend_Linear" 0.0 false))

(fn ConstructionScript
  (Transformation|SetWorldScale3D (Variables|Default|GetCineCamera) "1.000000,1.000000,1.000000"))