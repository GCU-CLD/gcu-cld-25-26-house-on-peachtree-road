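; CheckPoint_BP is a checkpoint trigger actor for a platform game that sets where the player spawns.
; On overlap by the player pawn, it stores its own location as PlayerSpawnLocation on BP_PlatformGame_PlayerController and changes its TextRender to a checkmark.
; A DoOnce gate runs before the player check, so only the first overlap by any actor is ever evaluated.
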(event EventBeginPlay)

(event Collision|EventActorBeginOverlap
  (params (OtherActor :type Actor%20Object%20Reference))
  (bind _returnvalue (Game|Player|GetPlayerPawn 0))
  (Utilities|FlowControl|DoOnce false
    (:Completed
      (if (== OtherActor _returnvalue)
        (Variables|/Game/PGTemplate/Blueprints/Characters/Player/BP_PlatformGame_PlayerController.BP_PlatformGame_PlayerController_C|SetPlayerSpawnLocation (.AsBP%20Platform%20Game%20Player%20Controller (Utilities|Casting|CastToBP_PlatformGame_PlayerController (Pawn|GetController _returnvalue))) (Transformation|GetActorLocation))
        (Rendering|Components|TextRender|SetText (Variables|Default|GetTextRender) (Utilities|Text|ToText(String) "✔"))))))

(fn ConstructionScript)