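; Trigger gate that sets how the player character moves when crossing it, based on the side it enters from.
; On overlap, it compares player and gate X positions to pick a directional gait, crouch or uncrouch, and optionally play a landing-roll montage.
; The gait selection maps LTR to the higher-X side, while the crouch and roll flags map LTR to the other side.
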(event EventBeginPlay)

(event Collision|EventActorBeginOverlap
  (params (OtherActor :type Actor%20Object%20Reference))
  (bind _asbp_player_character (Utilities|Casting|CastToBP_PlayerCharacter OtherActor))
  (Default|SetDesiredMovementGait _asbp_player_character (select (> (.x (Transformation|GetActorLocation _asbp_player_character)) (.x (Transformation|GetActorLocation))) (Variables|Default|GetLTR_MovementGait) (Variables|Default|GetRTL_MovementGait)))
  (if (or (and (Variables|Default|GetLTR_ForceCrouch) (not (> (.x (Transformation|GetActorLocation _asbp_player_character)) (.x (Transformation|GetActorLocation))))) (and (Variables|Default|GetRTL_ForceCrouch) (> (.x (Transformation|GetActorLocation _asbp_player_character)) (.x (Transformation|GetActorLocation)))))
    (Character|Crouch _asbp_player_character)
    (else
      (Character|UnCrouch _asbp_player_character)))
  (if (or (and (Variables|Default|GetLTR_ForceRoll) (not (> (.x (Transformation|GetActorLocation _asbp_player_character)) (.x (Transformation|GetActorLocation))))) (and (Variables|Default|GetRTL_ForceRoll) (> (.x (Transformation|GetActorLocation _asbp_player_character)) (.x (Transformation|GetActorLocation)))))
    (Animation|PlayAnimMontage _asbp_player_character "/Game/PGTemplate/Blueprints/Characters/Core/Animations/ALS/ALS_N_LandRoll_F_UE5_Montage.ALS_N_LandRoll_F_UE5_Montage" 1.0 "None")))

(fn ConstructionScript)