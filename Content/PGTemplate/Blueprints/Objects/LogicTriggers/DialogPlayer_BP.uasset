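; DialogPlayer_BP is a switchable logic trigger that plays a sequence of dialog lines.
; Switchon passes a DoOnce, registers itself on the player character and shows each line as a DialogueBox_W widget with delay, image, text and sound.
; Lines needing input show a prompt, pause the game and swap to IMC_Dialog until NextLine restores IMC_Default.
; The last line or OnReset rewinds the index and re-arms the trigger.
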(event Custom|DisplayLine
  (bind _returnvalue (Game|GetPlayerController 0))
  (bind _lines (Variables|Default|GetLines))
  (bind _currentline (Variables|Default|GetCurrentLine))
  (bind _output (Utilities|Array|Get(acopy) _lines _currentline))
  (bind _returnvalue_2 (PlayerController|LocalPlayerSubsystems|GetEnhancedInputLocalPlayerSubsystem _returnvalue))
  (Utilities|FlowControl|Delay (.delaybeforeshowing _output))
  (bind _returnvalue_3 (UserInterface|CreateWidget "/Game/PGTemplate/UI/DialogueBox_W.DialogueBox_W_C" 0 (.imagetouse _output) (.text _output) (.displaytime _output) (.soundcuetoplay _output)))
  (bind _output_get (Variables|Default|SetCurrentDialogBox _returnvalue_3))
  (UserInterface|Viewport|AddtoViewport _output_get 0)
  (Utilities|FlowControl|Delay (.displaytime _output))
  (if (.waitforinput _output)
    (Widget|SetVisibility (Variables|/Game/PGTemplate/UI/DialogueBox_W.DialogueBox_W_C|GetPrompt (Variables|Default|GetCurrentDialogBox)) "Visible")
    (Game|SetGamePaused true)
    (Class|EnhancedInputSubsystemInterface|ClearAllMappings _returnvalue_2)
    (Input|AddMappingContext _returnvalue_2 "/Game/PGTemplate/Blueprints/Characters/Player/Input/IMC_Dialog.IMC_Dialog" 0 "(bIgnoreAllPressedKeysUntilRelease=True,bForceImmediately=False,bNotifyUserSettings=False)")
    (else
      (CallFunction|NextLine))))

(event Custom|NextLine
  (bind _returnvalue (Game|GetPlayerController 0))
  (bind _returnvalue_2 (PlayerController|LocalPlayerSubsystems|GetEnhancedInputLocalPlayerSubsystem _returnvalue))
  (Class|EnhancedInputSubsystemInterface|ClearAllMappings _returnvalue_2)
  (Input|AddMappingContext _returnvalue_2 "/Game/PGTemplate/Blueprints/Characters/Player/Input/IMC_Default.IMC_Default" 0 "(bIgnoreAllPressedKeysUntilRelease=True,bForceImmediately=False,bNotifyUserSettings=False)")
  (Game|SetGamePaused false)
  (Widget|RemovefromParent (Variables|Default|GetCurrentDialogBox))
  (bind _result (Math|Integer|IncrementInt (Variables|Default|GetCurrentLine))
    (:%20%20
      (if (< _result (Utilities|Array|Length (Variables|Default|GetLines)))
        (CallFunction|DisplayLine)
        (else
          (Variables|Default|SetCurrentLine 0)
          (CallFunction|Reset))))))

(event Custom|Reset
  (Utilities|FlowControl|DoOnce false) ; enters at Reset
)

(event EventBeginPlay)

(event Collision|EventActorBeginOverlap
  (params (OtherActor :type Actor%20Object%20Reference)))

(event EventTick
  (params (DeltaSeconds :type Float%20%28single-precision%29)))

(event EventSwitchon
  (Utilities|FlowControl|DoOnce false
    (:Completed
      (Variables|/Game/PGTemplate/Blueprints/Characters/Player/BP_PlayerCharacter.BP_PlayerCharacter_C|SetCurrentDialogPlayer (.AsBP%20Player%20Character (Utilities|Casting|CastToBP_PlayerCharacter (Game|Player|GetPlayerPawn 0))) self)
      (CallFunction|DisplayLine))))

(event EventOnReset
  (Variables|Default|SetCurrentLine 0)
  (CallFunction|Reset))

(fn ConstructionScript)

(fn GetStatus
  (return false))