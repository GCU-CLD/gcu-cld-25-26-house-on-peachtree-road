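; Base interactive object that the player character can detect, interact with and look at when highlighted.
; PlayerDetection overlaps add it to or remove it from the player's interactive list, skipping adding while carried; Interact makes it the instigator's current object.
; Highlighting toggles custom depth on all static meshes, tints the camera manager's post-process outline and drives the character's look-at alpha.
; The construction script positions the look-at point from LookAtTarget.
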(event OnComponentBeginOverlap(PlayerDetection)
  (params (OverlappedComponent :type Primitive%20Component%20Object%20Reference) (OtherActor :type Actor%20Object%20Reference) (OtherComp :type Primitive%20Component%20Object%20Reference) (OtherBodyIndex :type Integer) (bFromSweep :type Boolean) (SweepResult :type Hit%20Result%20Structure%20%28by%20ref%29))
  (bind _self self)
  (bind _asbp_player_character (Utilities|Casting|CastToBP_PlayerCharacter OtherActor))
  (if (!= (Variables|/Game/PGTemplate/Blueprints/Characters/Core/BP_PlatformGameCharacter.BP_PlatformGameCharacter_C|GetCurrentlyCarriedObject _asbp_player_character) _self)
    (Default|AddNewInteractiveObject _asbp_player_character _self)))

(event OnComponentEndOverlap(PlayerDetection)
  (params (OverlappedComponent :type Primitive%20Component%20Object%20Reference) (OtherActor :type Actor%20Object%20Reference) (OtherComp :type Primitive%20Component%20Object%20Reference) (OtherBodyIndex :type Integer))
  (bind _asbp_player_character (Utilities|Casting|CastToBP_PlayerCharacter OtherActor))
  (Default|RemoveInteractiveObject _asbp_player_character self))

(event Custom|Interact
  (params (InstigatingCharacter :type BP%20Platform%20Game%20Character%20Object%20Reference))
  (Variables|/Game/PGTemplate/Blueprints/Characters/Player/BP_PlayerCharacter.BP_PlayerCharacter_C|SetCurrentInteractiveObject InstigatingCharacter self))

(event Custom|Highlight
  (params (Character :type BP%20Platform%20Game%20Character%20Object%20Reference) (HighlightColor :type Linear%20Color%20Structure))
  (for _array_element (Actor|GetComponentsByClass "/Script/Engine.StaticMeshComponent")
    (Rendering|SetRenderCustomDepth _array_element true)
    (Rendering|Material|SetVectorParameterValue (.AsMaterial%20Instance%20Dynamic (Utilities|Casting|CastToMaterialInstanceDynamic (Variables|/Game/PGTemplate/Blueprints/Characters/Player/BP_PlatformGameCameraManager.BP_PlatformGameCameraManager_C|GetDynamicPostProcessMaterial (.AsBP%20Platform%20Game%20Camera%20Manager (Utilities|Casting|CastToBP_PlatformGameCameraManager (Game|GetPlayerCameraManager 0)))))) "OutlineColor" HighlightColor :!class /Script/Engine.MaterialInstanceDynamic)
    (Variables|/Game/PGTemplate/Blueprints/Characters/Player/BP_PlayerCharacter.BP_PlayerCharacter_C|SetLookAtTargetWorld Character (Transformation|GetWorldLocation (Variables|Default|GetLookAtTargetPosition)))
    (Variables|/Game/PGTemplate/Blueprints/Characters/Player/BP_PlayerCharacter.BP_PlayerCharacter_C|SetLookAtAlpha Character 1.0)))

(event Custom|DeHighlight
  (params (Character :type BP%20Platform%20Game%20Character%20Object%20Reference))
  (for _array_element (Actor|GetComponentsByClass "/Script/Engine.StaticMeshComponent")
    (Rendering|SetRenderCustomDepth _array_element false)
    (Variables|/Game/PGTemplate/Blueprints/Characters/Player/BP_PlayerCharacter.BP_PlayerCharacter_C|SetLookAtAlpha Character 0.0)))

(event EventBeginPlay)

(event Collision|EventActorBeginOverlap
  (params (OtherActor :type Actor%20Object%20Reference)))

(event EventTick
  (params (DeltaSeconds :type Float%20%28single-precision%29)))

(fn ConstructionScript
  (Transformation|SetRelativeLocation (Variables|Default|GetLookAtTargetPosition) (Variables|Default|GetLookAtTarget) false false))