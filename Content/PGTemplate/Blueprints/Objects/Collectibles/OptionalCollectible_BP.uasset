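; OptionalCollectible_BP is an optional pickup in the platform game template that the player collects by touch.
; On Tick it bobs MeshRoot vertically with a time-based sine offset and spins it by a fixed step, both applied per frame without delta-time scaling.
; When the player pawn overlaps the Mesh, it notifies BP_PlatformGame_GameMode of the collection and destroys itself.
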(event OnComponentBeginOverlap(Mesh)
  (params (OverlappedComponent :type Primitive%20Component%20Object%20Reference) (OtherActor :type Actor%20Object%20Reference) (OtherComp :type Primitive%20Component%20Object%20Reference) (OtherBodyIndex :type Integer) (bFromSweep :type Boolean) (SweepResult :type Hit%20Result%20Structure%20%28by%20ref%29))
  (if (== OtherActor (Game|Player|GetPlayerPawn 0))
    (Default|OptionalCollectibleCollected (.AsBP%20Platform%20Game%20Game%20Mode (Utilities|Casting|CastToBP_PlatformGame_GameMode (Game|GetGameMode))))
    (Actor|DestroyActor)))

(event EventBeginPlay)

(event Collision|EventActorBeginOverlap
  (params (OtherActor :type Actor%20Object%20Reference)))

(event EventTick
  (params (DeltaSeconds :type Float%20%28single-precision%29))
  (bind _meshroot (Variables|Default|GetMeshRoot))
  (Transformation|AddRelativeLocation _meshroot (Math|Vector|MakeVector 0.0 0.0 (* (Math|Trig|Sin(Degrees) (* (Utilities|Time|GetTimeSeconds) 175.0)) 1.5)) false false)
  (Transformation|AddRelativeRotation _meshroot "0.000000,5.000000,0.000000" false false))

(fn ConstructionScript)