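; Interactable collectible object that the player character picks up into the inventory.
; Interact blocks control, crouches for low items and plays a right-hand pickup montage with a motion warp target at the item.
; A timeline moves the right-hand IK anchor from item to hip and updates look-at, then restores control and adds the item.
; Reset detaches the object, restores mesh and detection, and clears the HUD inventory.
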(event EventBeginPlay
  (bind _collectiblemesh (Variables|Default|GetCollectibleMesh))
  (|CallParentFunction)
  (Variables|Default|SetStartingLocation (Variables|/Script/Engine.SceneComponent|GetRelativeLocation _collectiblemesh))
  (Variables|Default|SetStartingRotation (Variables|/Script/Engine.SceneComponent|GetRelativeRotation _collectiblemesh)))

(event Collision|EventActorBeginOverlap
  (params (OtherActor :type Actor%20Object%20Reference))
  (|CallParentFunction OtherActor) ; This node is disabled and will not be called.\nDrag off pins to build functionality.
)

(event EventTick
  (params (DeltaSeconds :type Float%20%28single-precision%29))
  (|CallParentFunction DeltaSeconds) ; This node is disabled and will not be called.\nDrag off pins to build functionality.
)

(event EventInteract
  (params (InstigatingCharacter :type BP%20Platform%20Game%20Character%20Object%20Reference))
  (|CallParentFunction InstigatingCharacter)
  (Default|BlockControl InstigatingCharacter false)
  (if (> (- (.z (Transformation|GetActorLocation InstigatingCharacter)) (.z (Transformation|GetWorldLocation (Variables|Default|GetCollectibleMesh)))) 5e+01)
    (Character|Crouch InstigatingCharacter))
  (Class|MotionWarpingComponent|AddorUpdateWarpTarget (Variables|/Game/PGTemplate/Blueprints/Characters/Core/BP_PlatformGameCharacter.BP_PlatformGameCharacter_C|GetMotionWarping InstigatingCharacter) (Utilities|Struct|MakeMotionWarpingTarget "Target" (Math|Vector|MakeVector (.x (Transformation|GetWorldLocation (Variables|Default|GetCollectibleMesh))) 0.0 0.0)))
  (Animation|PlayAnimMontage InstigatingCharacter "/Game/PGTemplate/Blueprints/Characters/Core/Animations/Mixamo/Interactions/PickupObject_R_Montage.PickupObject_R_Montage" 3.0 "None")
  (bind _alphaitemtohip (Timeline|UpdateIKTarget Play)
    (:Update
      (if true
        (Variables|/Game/PGTemplate/Blueprints/Characters/Core/BP_PlatformGameCharacter.BP_PlatformGameCharacter_C|SetHandAnchorRight InstigatingCharacter (Math|Vector|SelectVector (+ (Transformation|GetSocketLocation (Variables|/Script/Engine.Character|GetMesh InstigatingCharacter) "pelvis") (Math|Vector|RotateVector (Math|Vector|SelectVector "0.000000,20.000000,0.000000" "0.000000,-20.000000,0.000000" true) (Transformation|GetActorRotation InstigatingCharacter))) (Transformation|GetWorldLocation (Variables|Default|GetCollectibleMesh)) (> _alphaitemtohip 0.5)))
        (else
          (Variables|/Game/PGTemplate/Blueprints/Characters/Core/BP_PlatformGameCharacter.BP_PlatformGameCharacter_C|SetHandAnchorLeft InstigatingCharacter (Math|Vector|SelectVector (+ (Transformation|GetSocketLocation (Variables|/Script/Engine.Character|GetMesh InstigatingCharacter) "pelvis") (Math|Vector|RotateVector (Math|Vector|SelectVector "0.000000,20.000000,0.000000" "0.000000,-20.000000,0.000000" true) (Transformation|GetActorRotation InstigatingCharacter))) (Transformation|GetWorldLocation (Variables|Default|GetCollectibleMesh)) (> _alphaitemtohip 0.5)))))
      (Variables|/Game/PGTemplate/Blueprints/Characters/Core/BP_PlatformGameCharacter.BP_PlatformGameCharacter_C|SetLookAtTargetWorld InstigatingCharacter (Transformation|GetWorldLocation (Variables|Default|GetCollectibleMesh))))
    (:Finished
      (Character|UnCrouch InstigatingCharacter)
      (Default|UnBlockControl InstigatingCharacter)
      (Components|Activation|Deactivate (Variables|Default|GetPlayerDetection))
      (Default|AddtoInventory InstigatingCharacter self))))

(event EventOnReset
  (bind _collectiblemesh (Variables|Default|GetCollectibleMesh))
  (Transformation|DetachFromActor "KeepRelative" "KeepRelative" "KeepRelative")
  (Components|Activation|Activate (Variables|Default|GetPlayerDetection) true)
  (Transformation|AttachComponentToComponent _collectiblemesh (Variables|Transformation|GetRootComponent) "None" "SnapToTarget" "SnapToTarget" "KeepWorld" true)
  (Transformation|SetRelativeLocationAndRotation _collectiblemesh (Variables|Default|GetStartingLocation) (Variables|Default|GetStartingRotation) false false)
  (Rendering|SetVisibility _collectiblemesh true false)
  (bind _asbp_platform_game_game_mode (Utilities|Casting|CastToBP_PlatformGame_GameMode (Game|GetGameMode)))
  (Default|ClearInventory (Variables|/Game/PGTemplate/Blueprints/Core/BP_PlatformGame_GameMode.BP_PlatformGame_GameMode_C|GetPlayerHUD _asbp_platform_game_game_mode)))

(fn ConstructionScript
  (|CallParentFunction)
  (Transformation|SetWorldLocation (Variables|Default|GetLookAtTargetPosition) (Transformation|GetWorldLocation (Variables|Default|GetCollectibleMesh)) false false))