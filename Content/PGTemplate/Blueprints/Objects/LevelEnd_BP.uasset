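; LevelEnd_BP is the level exit door that ends the level when the player walks into it while it is open.
; Open runs once, setting IsOpen, playing a sound and swinging the Door with a timeline.
; A grounded player overlapping PlayerDetection gets a forced camera offset, disabled collision and plane constraint, and a motion-warped walk montage toward ExitPoint.
; When that montage blends out, the game mode's LevelComplete is called.
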(event OnComponentBeginOverlap(PlayerDetection)
  (params (OverlappedComponent :type Primitive%20Component%20Object%20Reference) (OtherActor :type Actor%20Object%20Reference) (OtherComp :type Primitive%20Component%20Object%20Reference) (OtherBodyIndex :type Integer) (bFromSweep :type Boolean) (SweepResult :type Hit%20Result%20Structure%20%28by%20ref%29))
  (bind _returnvalue (Game|Player|GetPlayerPawn 0))
  (if (Math|Boolean|ANDBoolean (== OtherActor _returnvalue) (Variables|Default|GetisOpen) (AI|Components|NavMovement|IsMovingonGround (Variables|/Script/Engine.Character|GetCharacterMovement (.AsBP%20Platform%20Game%20Character (Utilities|Casting|CastToBP_PlatformGameCharacter _returnvalue)))))
    (bind _asbp_player_character (Utilities|Casting|CastToBP_PlayerCharacter OtherActor))
    (Variables|/Game/PGTemplate/Blueprints/Characters/Core/BP_PlatformGameCharacter.BP_PlatformGameCharacter_C|SetForceCameraOffset _asbp_player_character true)
    (Variables|/Game/PGTemplate/Blueprints/Characters/Core/BP_PlatformGameCharacter.BP_PlatformGameCharacter_C|SetForcedCameraOffset _asbp_player_character "0.000000,500.000000,100.000000")
    (Variables|/Game/PGTemplate/Blueprints/Characters/Core/BP_PlatformGameCharacter.BP_PlatformGameCharacter_C|SetForcedCameraOffsetLerp _asbp_player_character 0.99)
    (Collision|SetActorEnableCollision _asbp_player_character false)
    (Pawn|Components|CharacterMovement|SetMovementMode (Variables|/Script/Engine.Character|GetCharacterMovement _asbp_player_character) "MOVE_Flying" 0)
    (Class|MotionWarpingComponent|AddorUpdateWarpTargetfromLocation (Variables|/Game/PGTemplate/Blueprints/Characters/Core/BP_PlatformGameCharacter.BP_PlatformGameCharacter_C|GetMotionWarping _asbp_player_character) "MoveTarget" (Transformation|GetWorldLocation (Variables|Default|GetExitPoint)))
    (Class|MovementComponent|SetPlaneConstraintEnabled (Pawn|GetMovementComponent _asbp_player_character) false)
    (Default|BlockControl _asbp_player_character false)
    (Animation|Montage|PlayMontage (Variables|/Script/Engine.Character|GetMesh _asbp_player_character) "/Game/PGTemplate/Blueprints/Characters/Core/Animations/Mixamo/Interactions/HappyWalk_UE_Montage.HappyWalk_UE_Montage"
      (:OnBlendOut
        (Default|LevelComplete (.AsBP%20Platform%20Game%20Game%20Mode (Utilities|Casting|CastToBP_PlatformGame_GameMode (Game|GetGameMode))))))))

(event Custom|Open
  (Utilities|FlowControl|DoOnce false
    (:Completed
      (Variables|Default|SetisOpen true)
      (Audio|PlaySoundatLocation "/Game/PGTemplate/Blueprints/Characters/Core/Audio/Door-Open_Cue.Door-Open_Cue" (Transformation|GetActorLocation) "0, 0, 0" 1.0 1.0 0.0 0 0 0 0)
      (bind _doorrotation (Timeline|Timeline PlayFromStart)
        (:Update
          (Transformation|SetRelativeRotation (Variables|Default|GetDoor) (Math|Rotator|MakeRotator 0.0 0.0 _doorrotation) false false))))))

(fn ConstructionScript)