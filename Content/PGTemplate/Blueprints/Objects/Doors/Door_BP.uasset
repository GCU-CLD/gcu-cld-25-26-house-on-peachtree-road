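; Switchable door Blueprint that swings open or closed in yaw and reports its open state through GetStatus.
; Switchon and SwitchOff play or reverse a rotation Timeline with a matching sound, acting only when the state changes.
; InvertBehaviour swaps the meaning of both events and of the initial status.
; SetInitialStatus jumps the Timeline to either end and applies that rotation without animation or sound.
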(event EventSwitchon
  (bind _returnvalue (Transformation|GetActorLocation))
  (if (Variables|Default|GetInvertBehaviour)
    (if (Variables|Default|GetisOpen)
      (Audio|PlaySoundatLocation "/Game/PGTemplate/Blueprints/Characters/Core/Audio/Door-Close_Cue.Door-Close_Cue" _returnvalue "0, 0, 0" 1.0 1.0 0.0 0 0 0 0)
      (Variables|Default|SetisOpen false)
      (bind _doorrotation (Timeline|Timeline Reverse)
        (:Update
          (Transformation|SetRelativeRotation (Variables|Default|GetDoor) (Math|Rotator|MakeRotator 0.0 0.0 _doorrotation) false false))))
    (elif (not (Variables|Default|GetisOpen))
      (Audio|PlaySoundatLocation "/Game/PGTemplate/Blueprints/Characters/Core/Audio/Door-Open_Cue.Door-Open_Cue" _returnvalue "0, 0, 0" 1.0 1.0 0.0 0 0 0 0)
      (Variables|Default|SetisOpen true)
      (Timeline|Timeline Play))))

(event EventSwitchOff
  (bind _returnvalue (Transformation|GetActorLocation))
  (if (Variables|Default|GetInvertBehaviour)
    (if (not (Variables|Default|GetisOpen))
      (Audio|PlaySoundatLocation "/Game/PGTemplate/Blueprints/Characters/Core/Audio/Door-Open_Cue.Door-Open_Cue" _returnvalue "0, 0, 0" 1.0 1.0 0.0 0 0 0 0)
      (Variables|Default|SetisOpen true)
      (bind _doorrotation (Timeline|Timeline Play)
        (:Update
          (Transformation|SetRelativeRotation (Variables|Default|GetDoor) (Math|Rotator|MakeRotator 0.0 0.0 _doorrotation) false false))))
    (elif (Variables|Default|GetisOpen)
      (Audio|PlaySoundatLocation "/Game/PGTemplate/Blueprints/Characters/Core/Audio/Door-Close_Cue.Door-Close_Cue" _returnvalue "0, 0, 0" 1.0 1.0 0.0 0 0 0 0)
      (Variables|Default|SetisOpen false)
      (Timeline|Timeline Reverse))))

(event EventSetInitialStatus
  (params (InitialStatus :type Boolean))
  (bind _timeline (Variables|Default|GetTimeline))
  (bind _output_get (Variables|Default|SetisOpen (select (Variables|Default|GetInvertBehaviour) (not InitialStatus) InitialStatus)))
  (Components|Timeline|SetNewTime _timeline (Math|Float|SelectFloat (Components|Timeline|GetTimelineLength _timeline) 0.0 _output_get))
  (Transformation|SetRelativeRotation (Variables|Default|GetDoor) (Math|Rotator|MakeRotator 0.0 0.0 (stale EventSwitchon _doorrotation)) false false))

(fn ConstructionScript)

(fn GetStatus
  (return (Variables|Default|GetisOpen)))