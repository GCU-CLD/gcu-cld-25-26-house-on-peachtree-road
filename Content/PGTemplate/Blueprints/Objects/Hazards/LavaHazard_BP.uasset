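; Lava hazard Blueprint, a child of a hazard parent class that adds lava effects when its hazard mesh is overlapped.
; It overrides HazardMeshOverlapActions to loop a random number of times, spawning the Lava_NS Niagara system at the impact position.
; The parent implementation is called inside that loop, so inherited overlap actions repeat with each spawn.
; The event graph and construction script add no logic of their own.
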(event EventBeginPlay
  (|CallParentFunction) ; This node is disabled and will not be called.\nDrag off pins to build functionality.
)

(event Collision|EventActorBeginOverlap
  (params (OtherActor :type Actor%20Object%20Reference))
  (|CallParentFunction OtherActor) ; This node is disabled and will not be called.\nDrag off pins to build functionality.
)

(event EventTick
  (params (DeltaSeconds :type Float%20%28single-precision%29))
  (|CallParentFunction DeltaSeconds) ; This node is disabled and will not be called.\nDrag off pins to build functionality.
)

(fn ConstructionScript
  (|CallParentFunction))

(fn HazardMeshOverlapActions
  (params (ImpactPosition :type Vector :default "0, 0, 0") (LaunchedVector :type Vector :default "0, 0, 0"))
  (for _index (range 0 (Math|Random|RandomIntegerinRange 3 8))
    (Niagara|SpawnSystematLocation "/Game/PGTemplate/Blueprints/Objects/Hazards/VFX/Lava_NS.Lava_NS" ImpactPosition)
    (|CallParentFunction ImpactPosition LaunchedVector)))