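; Spike hazard actor that lays a row of cone meshes along a spline and reacts to anything that overlaps them.
; The construction script spawns spikes at SpikeSize intervals along the spline, aligned to its tangent, with the chosen material and overlap-only collision responses.
; On BeginPlay it binds each spike's overlap event, which passes the other actor and sweep impact point and normal to ProcessHit.
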(event Custom|BoundOverlapEvent
  (params (OverlappedComponent :type Primitive%20Component%20Object%20Reference) (OtherActor :type Actor%20Object%20Reference) (OtherComp :type Primitive%20Component%20Object%20Reference) (OtherBodyIndex :type Integer) (bFromSweep :type Boolean) (SweepResult :type Hit%20Result%20Structure%20%28by%20ref%29))
  (CallFunction|ProcessHit OtherActor (.impactpoint SweepResult) (.impactnormal SweepResult)))

(event EventBeginPlay
  (|CallParentFunction)
  (for _array_element (Variables|Default|GetSpikes)
    (Collision|BindEventtoOnComponentBeginOverlap _array_element (delegate Custom|BoundOverlapEvent))))

(event Collision|EventActorBeginOverlap
  (params (OtherActor :type Actor%20Object%20Reference))
  (|CallParentFunction OtherActor) ; This node is disabled and will not be called.\nDrag off pins to build functionality.
)

(event EventTick
  (params (DeltaSeconds :type Float%20%28single-precision%29))
  (|CallParentFunction DeltaSeconds) ; This node is disabled and will not be called.\nDrag off pins to build functionality.
)

(fn ConstructionScript
  (bind _spline (Variables|Default|GetSpline))
  (|CallParentFunction)
  (for _index (range 0 (Math|Float|Truncate (/ (Spline|GetSplineLength (Variables|Default|GetSpline)) (Variables|Default|GetSpikeSize))))
    (bind _returnvalue (AddComponent|AddStaticMeshComponent false (Math|Transform|MakeTransform (Spline|GetLocationatDistanceAlongSpline _spline (* (Variables|Default|GetSpikeSize) _index) "Local") (Math|Rotator|MakeRotfromX (Spline|GetTangentatDistanceAlongSpline _spline (* (Variables|Default|GetSpikeSize) _index) "Local")) "1.000000,1.000000,1.000000")))
    (Components|StaticMesh|SetStaticMesh _returnvalue "/Engine/BasicShapes/Cone.Cone")
    (Collision|SetCollisionResponsetoAllChannels _returnvalue "ECR_Overlap")
    (Rendering|Material|SetMaterial _returnvalue 0 (Variables|Default|GetMaterial))
    (Utilities|Array|Add (Variables|Default|GetSpikes) _returnvalue)))