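; DecompressionHazard_BP is a hazard that sucks characters toward a vacuum point and kills them.
; On Detection overlap, it calls BlockControl on the player character, ragdolls it, adds it to TrappedCharacters and calls Die after a one-second delay.
; Each Tick applies a velocity-change impulse to every trapped mesh toward VacuumAttractionPoint, scaled by distance, and removes invalid entries from the list.
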(event OnComponentBeginOverlap(Detection)
  (params (OverlappedComponent :type Primitive%20Component%20Object%20Reference) (OtherActor :type Actor%20Object%20Reference) (OtherComp :type Primitive%20Component%20Object%20Reference) (OtherBodyIndex :type Integer) (bFromSweep :type Boolean) (SweepResult :type Hit%20Result%20Structure%20%28by%20ref%29))
  (bind _asbp_platform_game_character (Utilities|Casting|CastToBP_PlatformGameCharacter OtherActor)
    (:then
      (bind _asbp_player_character (Utilities|Casting|CastToBP_PlayerCharacter _asbp_platform_game_character))
      (Default|BlockControl _asbp_player_character false))
    (:CastFailed
      _))
  (Default|Ragdoll _asbp_platform_game_character)
  (Utilities|Array|Add (Variables|Default|GetTrappedCharacters) _asbp_platform_game_character)
  (Utilities|FlowControl|Delay 1.0)
  (Default|Die _asbp_platform_game_character))

(event EventTick
  (params (DeltaSeconds :type Float%20%28single-precision%29))
  (bind _trappedcharacters (Variables|Default|GetTrappedCharacters))
  (for _array_element _trappedcharacters
    (Utilities|IsValid _array_element
      (:Is%20Valid
        (Physics|AddImpulse (Variables|/Script/Engine.Character|GetMesh _array_element) (* (- (Transformation|GetWorldLocation (Variables|Default|GetVacuumAttractionPoint)) (Transformation|GetActorLocation _array_element)) (Math|Float|MakeLiteralFloat 1.0)) "None" true))
      (:Is%20Not%20Valid
        (Utilities|Array|RemoveItem _trappedcharacters _array_element)))))

(fn ConstructionScript)