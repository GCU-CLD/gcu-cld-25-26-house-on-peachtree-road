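; Environmental foreground prop that fades its mesh's opacity when the player character enters its Box trigger, and restores it on exit.
; The construction script creates a dynamic instance of ForegroundObject_M on the static mesh and applies the MeshTexture variable to it.
; Box overlaps play or reverse the LerpAlpha timeline, which drives that material's Opacity parameter.
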(event OnComponentBeginOverlap(Box)
  (params (OverlappedComponent :type Primitive%20Component%20Object%20Reference) (OtherActor :type Actor%20Object%20Reference) (OtherComp :type Primitive%20Component%20Object%20Reference) (OtherBodyIndex :type Integer) (bFromSweep :type Boolean) (SweepResult :type Hit%20Result%20Structure%20%28by%20ref%29))
  (Utilities|Casting|CastToBP_PlayerCharacter OtherActor)
  (bind _materialalpha (Timeline|LerpAlpha Play)
    (:Update
      (Rendering|Material|SetScalarParameterValue (Variables|Default|GetDynamicMeshMaterial) "Opacity" _materialalpha :!class /Script/Engine.MaterialInstanceDynamic))))

(event OnComponentEndOverlap(Box)
  (params (OverlappedComponent :type Primitive%20Component%20Object%20Reference) (OtherActor :type Actor%20Object%20Reference) (OtherComp :type Primitive%20Component%20Object%20Reference) (OtherBodyIndex :type Integer))
  (Utilities|Casting|CastToBP_PlayerCharacter OtherActor)
  (bind _materialalpha (Timeline|LerpAlpha Reverse)
    (:Update
      (Rendering|Material|SetScalarParameterValue (Variables|Default|GetDynamicMeshMaterial) "Opacity" _materialalpha :!class /Script/Engine.MaterialInstanceDynamic))))

(event EventBeginPlay)

(event Collision|EventActorBeginOverlap
  (params (OtherActor :type Actor%20Object%20Reference)))

(event EventTick
  (params (DeltaSeconds :type Float%20%28single-precision%29)))

(fn ConstructionScript
  (bind _returnvalue (Rendering|Material|CreateDynamicMaterialInstance "/Game/PGTemplate/Blueprints/Objects/Environmental/ForegroundObject_M.ForegroundObject_M" "None" "None" :!class /Script/Engine.KismetMaterialLibrary))
  (bind _output_get (Variables|Default|SetDynamicMeshMaterial _returnvalue))
  (Rendering|Material|SetMaterial (Variables|Default|GetStaticMesh) 0 _output_get)
  (Rendering|Material|SetTextureParameterValue (Variables|Default|GetDynamicMeshMaterial) "MeshTexture" (Variables|Default|GetMeshTexture)))