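; Wall-jump traversal actor that catches an overlapping platformer character, holds it on the wall, then launches it off.
; On overlap it releases any rope, blocks control, switches to Flying, traces hand anchors and plays a motion-warped hang montage.
; WallJump triggers a jump toward ExitPoint, while HangDelay expiry causes a drop.
; Both share the exit montage, whose blend-out restores falling and control before launching the character.
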(event OnComponentBeginOverlap(PlayerDetection)
  (params (OverlappedComponent :type Primitive%20Component%20Object%20Reference) (OtherActor :type Actor%20Object%20Reference) (OtherComp :type Primitive%20Component%20Object%20Reference) (OtherBodyIndex :type Integer) (bFromSweep :type Boolean) (SweepResult :type Hit%20Result%20Structure%20%28by%20ref%29))
  (bind _entrypoint (Variables|Default|GetEntryPoint))
  (bind _entrypoint_2 (Variables|Default|GetEntryPoint))
  (bind _exitpoint (Variables|Default|GetExitPoint))
  (bind _returnvalue (Transformation|GetWorldLocation _exitpoint))
  (bind _returnvalue_2 (Transformation|GetWorldLocation _entrypoint_2))
  ;[1 1 1] Make sure we're triggered by a NEW character
  (bind _asbp_platform_game_character (Utilities|Casting|CastToBP_PlatformGameCharacter OtherActor))
  (Utilities|IsValid (Variables|/Game/PGTemplate/Blueprints/Characters/Core/BP_PlatformGameCharacter.BP_PlatformGameCharacter_C|GetCurrentRope _asbp_platform_game_character)
    (:Is%20Valid
      (bind _asbp_player_character (Utilities|Casting|CastToBP_PlayerCharacter _asbp_platform_game_character))
      (Default|DetachfromRope _asbp_player_character))
    (:Is%20Not%20Valid
      _))
  (if (!= _asbp_platform_game_character (Variables|Default|GetCurrentCharacter))
    (Animation|StopAnimMontage _asbp_platform_game_character 0)
    ;[1 1 1] Grab the entry Z - we don't know what height the player will enter at
    (Variables|Default|SetCharacterEntryZ (- (.z (Transformation|GetActorLocation _asbp_platform_game_character)) (Components|Capsule|GetScaledCapsuleHalfHeight (Variables|/Script/Engine.Character|GetCapsuleComponent _asbp_platform_game_character))))
    ;[1 1 1] Assume we're dropping rather than jumping
    (Variables|Default|SetisWallJumping false)
    ;[1 1 1] Check we're not already playing an animation
    (if (not (Class|Character|IsPlayingRootMotion _asbp_platform_game_character))
      ;[1 1 1] Grab Char and have Char grab this
      (bind _output_get (Variables|Default|SetCurrentCharacter _asbp_platform_game_character))
      (Variables|/Game/PGTemplate/Blueprints/Characters/Core/BP_PlatformGameCharacter.BP_PlatformGameCharacter_C|SetCurrentWallJump _output_get self)
      ;[1 1 1] Block control on the character
      (Default|BlockControl (Variables|Default|GetCurrentCharacter) true)
      ;[1 1 1] Set MovementMode to Flying so we can alter Z with root motion
      (Pawn|Components|CharacterMovement|SetMovementMode (Variables|/Script/Engine.Character|GetCharacterMovement (Variables|Default|GetCurrentCharacter)) "MOVE_Flying" 0)
      ;[1 1 1] Set up the Entry Point Warp Target
      (Class|MotionWarpingComponent|AddorUpdateWarpTargetfromLocationandRotation (Variables|/Game/PGTemplate/Blueprints/Characters/Core/BP_PlatformGameCharacter.BP_PlatformGameCharacter_C|GetMotionWarping (Variables|Default|GetCurrentCharacter)) (Utilities|Name|MakeLiteralName "EntryPoint") (+ (Math|Vector|MakeVector (.x (Transformation|GetWorldLocation _entrypoint)) 0.0 (Variables|Default|GetCharacterEntryZ)) "0.000000,0.000000,20.000000") (Transformation|GetWorldRotation _entrypoint))
      ;[1 1 1] Set up Hand Anchors by tracing to the wall from the character
      (CallFunction|SetHandAnchors)
      (Animation|Montage|PlayMontage (Variables|/Script/Engine.Character|GetMesh (Variables|Default|GetCurrentCharacter)) "/Game/PGTemplate/Blueprints/Characters/Core/Animations/Custom/WallJumpWithIdle_Montage.WallJumpWithIdle_Montage" 1.25 0.0 "Default"
        (:then
          ;[1 1 1] Player doesn't initiate WallJump
          (Utilities|FlowControl|Delay (Variables|Default|GetHangDelay))
          (if (not (Variables|Default|GetisWallJumping)) ; Catch to prevent jump firing twice!
            (Variables|Default|SetActualLaunchVector (select (Variables|Default|GetisWallJumping) "-1000.000000,0.000000,600.000000" "-250.000000,0.000000,-200.000000"))
            (Class|MotionWarpingComponent|AddorUpdateWarpTargetfromLocationandRotation (Variables|/Game/PGTemplate/Blueprints/Characters/Core/BP_PlatformGameCharacter.BP_PlatformGameCharacter_C|GetMotionWarping (Variables|Default|GetCurrentCharacter)) (Utilities|Name|MakeLiteralName "ExitPoint") (Math|Vector|SelectVector (Math|Vector|MakeVector (.x _returnvalue) (.y _returnvalue) (+ (Variables|Default|GetCharacterEntryZ) 5e+01)) (Math|Vector|MakeVector (.x _returnvalue_2) (.y _returnvalue_2) (+ (Variables|Default|GetCharacterEntryZ) -1e+01)) (Variables|Default|GetisWallJumping)) (Transformation|GetWorldRotation _exitpoint))
            (Variables|/Game/PGTemplate/Blueprints/Characters/Core/BP_PlatformGameCharacter.BP_PlatformGameCharacter_C|SetCurrentWallJump (Variables|Default|GetCurrentCharacter) 0)
            (Animation|Montage|PlayMontage (Variables|/Script/Engine.Character|GetMesh (Variables|Default|GetCurrentCharacter)) "/Game/PGTemplate/Blueprints/Characters/Core/Animations/Custom/WallJumpWithIdle_Montage.WallJumpWithIdle_Montage" 1.5 0.0 "WallJumpOut"
              (:OnBlendOut
                (Pawn|Components|CharacterMovement|SetMovementMode (Variables|/Script/Engine.Character|GetCharacterMovement (Variables|Default|GetCurrentCharacter)) "MOVE_Falling" 0)
                (Default|UnBlockControl (Variables|Default|GetCurrentCharacter))
                (Audio|Components|Audio|Stop (Variables|Default|GetUpdateIKAnchors))
                (Character|LaunchCharacter (Variables|Default|GetCurrentCharacter) (Math|Vector|RotateVector (Variables|Default|GetActualLaunchVector) (Transformation|GetWorldRotation (Variables|Default|GetEntryPoint))) true true)
                ;[1 1 1] Delay clearing character to prevent drop-in
                (Utilities|FlowControl|Delay 0.2)
                (Variables|Default|SetCurrentCharacter 0)))))))))

(event Custom|WallJump
  (bind _entrypoint (Variables|Default|GetEntryPoint))
  (bind _characterentryz (Variables|Default|GetCharacterEntryZ))
  (bind _exitpoint (Variables|Default|GetExitPoint))
  (bind _returnvalue (Transformation|GetWorldLocation _exitpoint))
  (bind _returnvalue_2 (Transformation|GetWorldLocation _entrypoint))
  ;[1 1 1] Player Initiates WallJump
  (Variables|Default|SetisWallJumping true)
  (Variables|Default|SetActualLaunchVector (select (Variables|Default|GetisWallJumping) "-1000.000000,0.000000,600.000000" "-250.000000,0.000000,-200.000000"))
  (Class|MotionWarpingComponent|AddorUpdateWarpTargetfromLocationandRotation (Variables|/Game/PGTemplate/Blueprints/Characters/Core/BP_PlatformGameCharacter.BP_PlatformGameCharacter_C|GetMotionWarping (Variables|Default|GetCurrentCharacter)) (Utilities|Name|MakeLiteralName "ExitPoint") (Math|Vector|SelectVector (Math|Vector|MakeVector (.x _returnvalue) (.y _returnvalue) (+ _characterentryz 5e+01)) (Math|Vector|MakeVector (.x _returnvalue_2) (.y _returnvalue_2) (+ _characterentryz -1e+01)) (Variables|Default|GetisWallJumping)) (Transformation|GetWorldRotation _exitpoint))
  (Variables|/Game/PGTemplate/Blueprints/Characters/Core/BP_PlatformGameCharacter.BP_PlatformGameCharacter_C|SetCurrentWallJump (Variables|Default|GetCurrentCharacter) 0)
  (Animation|Montage|PlayMontage (Variables|/Script/Engine.Character|GetMesh (Variables|Default|GetCurrentCharacter)) "/Game/PGTemplate/Blueprints/Characters/Core/Animations/Custom/WallJumpWithIdle_Montage.WallJumpWithIdle_Montage" 1.5 0.0 "WallJumpOut"
    (:OnBlendOut
      (Pawn|Components|CharacterMovement|SetMovementMode (Variables|/Script/Engine.Character|GetCharacterMovement (Variables|Default|GetCurrentCharacter)) "MOVE_Falling" 0)
      (Default|UnBlockControl (Variables|Default|GetCurrentCharacter))
      (Audio|Components|Audio|Stop (Variables|Default|GetUpdateIKAnchors))
      (Character|LaunchCharacter (Variables|Default|GetCurrentCharacter) (Math|Vector|RotateVector (Variables|Default|GetActualLaunchVector) (Transformation|GetWorldRotation (Variables|Default|GetEntryPoint))) true true)
      ;[1 1 1] Delay clearing character to prevent drop-in
      (Utilities|FlowControl|Delay 0.2)
      (Variables|Default|SetCurrentCharacter 0))))

(fn ConstructionScript
  (bind _entrypoint (Variables|Default|GetEntryPoint))
  (bind _exitpoint (Variables|Default|GetExitPoint))
  (Variables|Default|SetEntryPointLocation (Math|Vector|MakeVector (.x (Variables|Default|GetEntryPointLocation)) 0.0 0.0))
  (Variables|Default|SetExitPointLocation (Math|Vector|MakeVector (.x (Variables|Default|GetExitPointLocation)) 0.0 0.0))
  (bind _returnvalue (AddComponent|AddArrowComponent true))
  (Transformation|AttachComponentToComponent _returnvalue _entrypoint "None" "SnapToTarget" "SnapToTarget" "KeepWorld" true)
  (Transformation|SetRelativeLocation _entrypoint (Variables|Default|GetEntryPointLocation) false false)
  (bind _returnvalue_2 (AddComponent|AddArrowComponent true))
  (Transformation|AttachComponentToComponent _returnvalue_2 _exitpoint "None" "SnapToTarget" "SnapToTarget" "KeepWorld" true)
  (Transformation|SetRelativeLocation _exitpoint (Variables|Default|GetExitPointLocation) false false))

(fn SetHandAnchors
  (bind _currentcharacter (Variables|Default|GetCurrentCharacter))
  (bind _currentcharacter_2 (Variables|Default|GetCurrentCharacter))
  (bind _returnvalue (Transformation|GetActorRotation _currentcharacter_2))
  (bind _mesh (Variables|/Script/Engine.Character|GetMesh _currentcharacter))
  (bind _returnvalue_2 (Transformation|GetSocketLocation _mesh "spine_05"))
  (bind _outhit (Collision|LineTraceByChannel _returnvalue_2 (+ _returnvalue_2 (* (Math|Vector|SelectVector "1.000000,0.000000,0.000000" "-1.000000,0.000000,0.000000" (< (/ (Math|Float|Absolute(Float) (.yaw (Transformation|GetActorRotation self))) 1.8e+02) 1.0)) (Math|Float|MakeLiteralFloat 1e+03))) "TraceTypeQuery1" false (Utilities|Array|MakeArray (Variables|Default|GetCurrentCharacter)) "None"))
  (if (.bblockinghit _outhit)
    (Variables|/Game/PGTemplate/Blueprints/Characters/Core/BP_PlatformGameCharacter.BP_PlatformGameCharacter_C|SetHandAnchorLeft _currentcharacter_2 (+ (.location _outhit) (Math|Vector|RotateVector "0.000000,-20.000000,20.000000" _returnvalue)))
    (Variables|/Game/PGTemplate/Blueprints/Characters/Core/BP_PlatformGameCharacter.BP_PlatformGameCharacter_C|SetHandAnchorRight _currentcharacter_2 (+ (.location _outhit) (Math|Vector|RotateVector "0.000000,20.000000,20.000000" _returnvalue)))
    (else
      (Development|PrintString (Utilities|String|Append "Hands do not hit wall on WallJump " (Utilities|GetDisplayName self))))))