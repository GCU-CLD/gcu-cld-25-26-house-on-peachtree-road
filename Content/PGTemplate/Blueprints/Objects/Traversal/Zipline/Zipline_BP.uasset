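; Zipline actor that carries the platformer character along a spline when it overlaps the trigger box.
; Construction tiles spline-mesh cable segments along the spline.
; Overlap blocks input, sets flying movement and plays a hang montage, then a length-scaled timeline moves the handle and offset character along the spline.
; At the end the character falls with input restored, but the stored rider is never cleared, so later overlaps are ignored.
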(event OnComponentBeginOverlap(Box)
  (params (OverlappedComponent :type Primitive%20Component%20Object%20Reference) (OtherActor :type Actor%20Object%20Reference) (OtherComp :type Primitive%20Component%20Object%20Reference) (OtherBodyIndex :type Integer) (bFromSweep :type Boolean) (SweepResult :type Hit%20Result%20Structure%20%28by%20ref%29))
  (bind _spline (Variables|Default|GetSpline))
  (Utilities|IsValid (Variables|Default|GetCurrentZipCharacter)
    (:Is%20Not%20Valid
      (bind _asbp_platform_game_character (Utilities|Casting|CastToBP_PlatformGameCharacter OtherActor))
      (bind _output_get (Variables|Default|SetCurrentZipCharacter _asbp_platform_game_character))
      (Variables|/Game/PGTemplate/Blueprints/Characters/Core/BP_PlatformGameCharacter.BP_PlatformGameCharacter_C|SetForceInputBlock _output_get true)
      (Pawn|Components|CharacterMovement|SetMovementMode (Variables|/Script/Engine.Character|GetCharacterMovement _asbp_platform_game_character) "MOVE_Flying" 0)
      (Animation|PlayAnimMontage (Variables|Default|GetCurrentZipCharacter) "/Game/PGTemplate/Blueprints/Objects/Traversal/Zipline/Animation/ZiplineHang_UE_Montage.ZiplineHang_UE_Montage" 1.0 "None")
      (Components|Timeline|SetPlayRate (Variables|Default|GetZiplineTimeline) (/ 1.0 (/ (/ (Spline|GetSplineLength (Variables|Default|GetSpline)) 1e+02) (Variables|Default|GetZipSpeed))))
      (Utilities|FlowControl|Delay 0.35)
      (bind _newtrack_0 (Timeline|ZiplineTimeline PlayFromStart)
        (:Update
          (Transformation|SetWorldLocation (Variables|Default|GetHandle) (Spline|GetLocationatDistanceAlongSpline _spline (* (Spline|GetSplineLength _spline) _newtrack_0) "World") false false)
          (Transformation|SetActorLocation (Variables|Default|GetCurrentZipCharacter) (- (Spline|GetLocationatDistanceAlongSpline _spline (* (Spline|GetSplineLength _spline) _newtrack_0) "World") "10.000000,0.000000,145.000000") false false))
        (:Finished
          (CallFunction|DetachPlayer))))))

(event Custom|DetachPlayer
  (bind _currentzipcharacter (Variables|Default|GetCurrentZipCharacter))
  (Variables|/Game/PGTemplate/Blueprints/Characters/Core/BP_PlatformGameCharacter.BP_PlatformGameCharacter_C|SetForceInputBlock _currentzipcharacter false)
  (Animation|StopAnimMontage _currentzipcharacter "/Game/PGTemplate/Blueprints/Objects/Traversal/Zipline/Animation/ZiplineHang_UE_Montage.ZiplineHang_UE_Montage")
  (Pawn|Components|CharacterMovement|SetMovementMode (Variables|/Script/Engine.Character|GetCharacterMovement _currentzipcharacter) "MOVE_Falling" 0))

(event EventBeginPlay)

(event Collision|EventActorBeginOverlap
  (params (OtherActor :type Actor%20Object%20Reference)))

(event EventTick
  (params (DeltaSeconds :type Float%20%28single-precision%29)))

(fn ConstructionScript
  (bind _spline (Variables|Default|GetSpline))
  (bind _spline_2 (Variables|Default|GetSpline))
  (bind _pipelength (LocalVariables|GetPipelength))
  (bind _relativelocation (Variables|/Script/Engine.SceneComponent|GetRelativeLocation _spline))
  (for _index (range 0 (- (Math|Float|Truncate (/ (Spline|GetSplineLength (Variables|Default|GetSpline)) (LocalVariables|GetPipelength))) 1))
    (bind _returnvalue (AddComponent|AddSplineMeshComponent false))
    (Components|StaticMesh|SetStaticMesh _returnvalue "/Game/PGTemplate/Blueprints/Objects/Switches/Meshes/cable.cable")
    (SplineMesh|SetStartandEnd _returnvalue (+ _relativelocation (Spline|GetLocationatDistanceAlongSpline _spline_2 (* _index _pipelength) "Local")) (Spline|GetTangentatDistanceAlongSpline _spline_2 (* _index _pipelength) "Local") (+ _relativelocation (Spline|GetLocationatDistanceAlongSpline _spline_2 (* (+ _index 1) _pipelength) "Local")) (Spline|GetTangentatDistanceAlongSpline _spline_2 (* (+ _index 1) _pipelength) "Local") true :!class /Script/Engine.SplineMeshComponent)))