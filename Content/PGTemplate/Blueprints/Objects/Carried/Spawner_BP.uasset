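; Interactable spawner that, when a character pushes its button, spawns an object of a configurable class above its plate, destroying the previous one.
; Spawning requires the spawner to be switched on and its spawn space clear, checked every Tick and shown by a green or red dynamic button material.
; Interaction plays a side-dependent hand-anchored push montage with optional crouch, while a timeline scales the new object's mesh.
; Player overlap toggles highlighting.
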(event OnComponentBeginOverlap(PlayerDetection)
  (params (OverlappedComponent :type Primitive%20Component%20Object%20Reference) (OtherActor :type Actor%20Object%20Reference) (OtherComp :type Primitive%20Component%20Object%20Reference) (OtherBodyIndex :type Integer) (bFromSweep :type Boolean) (SweepResult :type Hit%20Result%20Structure%20%28by%20ref%29))
  (bind _asbp_player_character (Utilities|Casting|CastToBP_PlayerCharacter OtherActor))
  (CallFunction|Highlight _asbp_player_character "(R=1.000000,G=0.000000,B=1.000000,A=1.000000)"))

(event OnComponentEndOverlap(PlayerDetection)
  (params (OverlappedComponent :type Primitive%20Component%20Object%20Reference) (OtherActor :type Actor%20Object%20Reference) (OtherComp :type Primitive%20Component%20Object%20Reference) (OtherBodyIndex :type Integer))
  (bind _asbp_player_character (Utilities|Casting|CastToBP_PlayerCharacter OtherActor))
  (CallFunction|DeHighlight _asbp_player_character))

(event EventBeginPlay)

(event EventSwitchon
  (if (not (Variables|Default|GetisActive))
    (Variables|Default|SetisActive true)
    (Rendering|Material|SetVectorParameterValue (Variables|Default|GetButtonMaterial) "Colour" "(R=0.000000,G=1.000000,B=0.000000,A=1.000000)" :!class /Script/Engine.MaterialInstanceDynamic)))

(event EventSwitchOff
  (if (Variables|Default|GetisActive)
    (Variables|Default|SetisActive false)
    (Rendering|Material|SetVectorParameterValue (Variables|Default|GetButtonMaterial) "Colour" "(R=1.000000,G=0.000000,B=0.000000,A=1.000000)" :!class /Script/Engine.MaterialInstanceDynamic)))

(event EventInteract
  (params (InstigatingCharacter :type BP%20Platform%20Game%20Character%20Object%20Reference))
  (bind _plate (Variables|Default|GetPlate))
  (bind _returnvalue (Transformation|GetWorldLocation _plate))
  (bind _returnvalue_2 (+ _returnvalue "0.000000,0.000000,50.000000"))
  (|PushButtonAnim InstigatingCharacter)
  (if (and (Variables|Default|GetisActive) (not (Variables|Default|GetspawnBlocked)))
    (Utilities|IsValid (Variables|Default|GetSpawnedObject)
      (:Is%20Valid
        (Default|Destroy (Variables|Default|GetSpawnedObject)))
      (:Is%20Not%20Valid
        _))
    (bind _returnvalue_3 (Game|SpawnActorfromClass (Variables|Default|GetObjectSpawnClass) (Math|Transform|MakeTransform _returnvalue_2 "0, 0, 0" "1.000000,1.000000,1.000000") "Undefined" "MultiplyWithRoot" 0 0))
    (Audio|PlaySoundatLocation "/Game/PGTemplate/Blueprints/Objects/Carried/Audio/CrateSpawn_Cue.CrateSpawn_Cue" _returnvalue_2 "0, 0, 0" 1.0 1.0 0.0 0 0 0 0)
    (Variables|Default|SetSpawnedObject _returnvalue_3)
    (bind _newtrack_0 (Timeline|ScaleAnimation PlayFromStart)
      (:Update
        (Transformation|SetWorldScale3D (Variables|/Game/PGTemplate/Blueprints/Objects/Carried/Core/CarriedObject_IO.CarriedObject_IO_C|GetMesh (Variables|Default|GetSpawnedObject)) (Math|Conversions|ToVector(Float) _newtrack_0))))))

(event EventTick
  (params (DeltaSeconds :type Float%20%28single-precision%29))
  (bind _buttonmaterial (Variables|Default|GetButtonMaterial))
  (if (> (Utilities|Array|Length (Collision|GetOverlappingActors (Variables|Default|GetSpawnSpace) 0 :!class /Script/Engine.PrimitiveComponent)) 1)
    (Variables|Default|SetspawnBlocked true)
    (Rendering|Material|SetVectorParameterValue _buttonmaterial "Colour" "(R=1.000000,G=0.000000,B=0.000000,A=1.000000)" :!class /Script/Engine.MaterialInstanceDynamic)
    (else
      (Variables|Default|SetspawnBlocked false)
      (if (Variables|Default|GetisActive)
        (Rendering|Material|SetVectorParameterValue _buttonmaterial "Colour" "(R=0.000000,G=1.000000,B=0.000000,A=1.000000)" :!class /Script/Engine.MaterialInstanceDynamic)))))

(fn ConstructionScript
  (bind _returnvalue (Rendering|Material|CreateDynamicMaterialInstance "/Game/PGTemplate/Environments/Materials/BasicColouredMaterial_M.BasicColouredMaterial_M" "None" "None" :!class /Script/Engine.KismetMaterialLibrary))
  (bind _output_get (Variables|Default|SetButtonMaterial _returnvalue))
  (Rendering|Material|SetVectorParameterValue _output_get "Colour" "(R=0.000000,G=1.000000,B=0.000000,A=1.000000)" :!class /Script/Engine.MaterialInstanceDynamic)
  (Rendering|Material|SetMaterial (Variables|Default|GetButtonIndicator) 0 (Variables|Default|GetButtonMaterial))
  (Components|StaticMesh|SetStaticMesh (Variables|Default|GetNiagaraPreviewMesh) (Variables|Default|GetPreviewMesh)))

(fn GetStatus
  (return false))