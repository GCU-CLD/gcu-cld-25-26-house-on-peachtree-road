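; Game mode for the main menu that sets up the menu screen and camera when play begins.
; On BeginPlay it creates the MenuScreen_W widget, adds it to the viewport and switches input to UI only, focusing the first child of its level entry container.
; It also shows the mouse cursor and sets the player's view to the first CineCameraActor found in the level.
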(event EventBeginPlay
  (bind _returnvalue (Game|GetPlayerController 0))
  (bind _returnvalue_2 (UserInterface|CreateWidget "/Game/PGTemplate/Maps/Menu/MenuScreen_W.MenuScreen_W_C" _returnvalue))
  (UserInterface|Viewport|AddtoViewport _returnvalue_2 0)
  (Input|SetInputModeUIOnly _returnvalue (Class|PanelWidget|GetChildat (Variables|/Game/PGTemplate/Maps/Menu/MenuScreen_W.MenuScreen_W_C|GetLevelEntryContainer _returnvalue_2)) "DoNotLock" false)
  (Variables|/Script/Engine.PlayerController|SetbShowMouseCursor _returnvalue true)
  (bind _outactors (Actor|GetAllActorsOfClass "/Script/CinematicCamera.CineCameraActor"))
  (Game|Player|SetViewTargetwithBlend (Game|GetPlayerController 0) (Utilities|Array|Get(acopy) _outactors) 0.0 "VTBlend_Linear" 0.0 false))

(event EventTick
  (params (DeltaSeconds :type Float%20%28single-precision%29)))

(fn ConstructionScript)