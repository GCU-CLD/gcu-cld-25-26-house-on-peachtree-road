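; Geometry Script generator actor that builds a platform mesh, flat or sloped, from end, height and depth vectors.
; On rebuild, it triangulates a four-point side profile, linearly extrudes it to twice the depth and shifts the pivot along Y by the depth.
; The construction script constrains each vector to its relevant axes, keeping height at or below a negative minimum thickness and depth non-negative.
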(event EventBeginPlay)

(event Collision|EventActorBeginOverlap
  (params (OtherActor :type Actor%20Object%20Reference)))

(event EventTick
  (params (DeltaSeconds :type Float%20%28single-precision%29)))

(event Events|EventOnRebuildGeneratedMesh
  (params (TargetMesh :type Dynamic%20Mesh%20Object%20Reference))
  (bind _platformheight (Variables|Default|GetPlatformHeight))
  (bind _platformend (Variables|Default|GetPlatformEnd))
  (bind _returnvalue (Class|GeometryScriptLibraryMeshPrimitiveFunctions|AppendTriangulatedPolygon :TargetMesh TargetMesh :Transform (Math|Transform|MakeTransform "0, 0, 0" "0.000000,0.000000,-90.000000" "1.000000,1.000000,1.000000") :PolygonVertices (Utilities|Array|MakeArray "" (Math|Vector2D|MakeVector2D 0.0 (.z _platformheight)) (Math|Vector2D|MakeVector2D (.x _platformend) (+ (.z _platformend) (.z _platformheight))) (Math|Vector2D|MakeVector2D (.x _platformend) (.z _platformend))) :Debug 0))
  (bind (_selection _returnvalue_2) (Class|GeometryScriptLibraryMeshSelectionFunctions|CreateSelectAllMeshSelection _returnvalue "Triangles"))
  (bind _returnvalue_3 (Class|GeometryScriptLibraryMeshModelingFunctions|ApplyMeshLinearExtrudeFaces _returnvalue_2 (Utilities|Struct|MakeGeometryScriptMeshLinearExtrudeOptions (* (.y (Variables|Default|GetPlatformDepth)) -2.0) "FixedDirection" "0.000000,-1.000000,0.000000" "EntireSelection" (Utilities|Struct|MakeGeometryScriptMeshEditPolygroupOptions "PreserveExisting")) _selection 0))
  (Class|GeometryScriptLibraryMeshTransformFunctions|TranslatePivottoLocation _returnvalue_3 (Math|Vector|MakeVector 0.0 (.y (Variables|Default|GetPlatformDepth)) 0.0) 0))

(fn ConstructionScript
  (Variables|Default|SetPlatformEnd (Math|Vector|MakeVector (.x (Variables|Default|GetPlatformEnd)) 0.0 (.z (Variables|Default|GetPlatformEnd))))
  (Variables|Default|SetPlatformHeight (Math|Vector|MakeVector 0.0 0.0 (Math|Float|SelectFloat -5.0 (.z (Variables|Default|GetPlatformHeight)) (> (.z (Variables|Default|GetPlatformHeight)) -5.0))))
  (Variables|Default|SetPlatformDepth (Math|Vector|MakeVector 0.0 (Math|Float|SelectFloat 0.0 (.y (Variables|Default|GetPlatformDepth)) (< (.y (Variables|Default|GetPlatformDepth)) 0.0)) 0.0)))